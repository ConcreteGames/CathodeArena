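; Utility Blueprint that applies automatic scalability settings once, unless a forced update is requested.
; SetScalabilityAuto uses the existence of a "ScalabilityAuto" save slot as a first-run flag, writing a Save_Scalability object there.
; It then waits the given number of frames and runs the "Scalability Auto" console command.
; BeginPlay is empty, so the event relies on an outside caller; leftover auto-trigger chains are disconnected.
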(event `self.ReceiveBeginPlay`)

(event `SetScalabilityAuto`
  (params (ForceUpdate :type Boolean :default false) (FramesDelay :type Integer :default 30))
  (bind _returnvalue (`GameplayStatics.DoesSaveGameExist` "ScalabilityAuto"))
  (if (or (not _returnvalue) ForceUpdate)
    (bind _returnvalue_2 (`GameplayStatics.CreateSaveGameObject` "/Game/ConcreteTemplate/Utility/ScalabilityAuto/Save_Scalability.Save_Scalability_C"))
    (`GameplayStatics.SaveGameToSlot` _returnvalue_2 "ScalabilityAuto")
    (`LowEntryExtendedStandardLibrary.DelayFrames` FramesDelay)
    (`KismetSystemLibrary.ExecuteConsoleCommand` "Scalability Auto" null)
    (`KismetSystemLibrary.PrintString` "Scalability Done")))

(fn `UserConstructionScript`)