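; Environment particle cannon actor whose Niagara effect intensifies with a "Bordel" amount.
; The Bordel event calls ParticlesStates, which remaps the amount to shorter lifetime, higher spawn rate and faster velocity through Niagara user parameters.
; ChangeNiagaraSystem swaps the effect asset, though the threshold-based swap logic is unconnected.
; The P key toggles the effect's visibility.
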(event `Key|P`
  (params (Key :type "Key Structure"))
  (:`Pressed`
    (bind _isa (`/Engine/EditorBlueprintResources/StandardMacros.FlipFlop`)
      (:`A`
        _)
      (:`B`
        _))
    (`SceneComponent.SetHiddenInGame` (`self.Fx`) _isa false)))

(event `self.ReceiveBeginPlay`)

(event `ChangeNiagaraSystem`
  (params (NiagaraSystem :type "NiagaraSystem Object Reference"))
  ;[1 1 1] Change Niagara System
  (set `self.NiagaraSystem` NiagaraSystem)
  (`NiagaraComponent.SetAsset` (`self.Fx`) (`self.NiagaraSystem`)))

(event `/Game/CathodeArena/Core/Engine/BPI_Game.Bordel`
  (params (BordelAmount :type Integer))
  ;[1 1 1] Add Bordel
  (`self.ParticlesStates` BordelAmount))

(fn `ParticlesStates`
  (params (Bordel :type Integer))
  (bind _fx (`self.Fx`))
  (bind _returnvalue (`KismetMathLibrary.Conv_IntToDouble` (`local.Bordel`)))
  (set `self.ParticlesLifetime` (`KismetMathLibrary.MapRangeClamped` _returnvalue 0.0 100.0 10.0 0.3))
  (set `self.ParticlesSpawnRate` (`KismetMathLibrary.MapRangeClamped` _returnvalue 0.0 100.0 10.0 5000.0))
  (set `self.ParticlesVelocity` (`KismetMathLibrary.MapRangeClamped` _returnvalue 0.0 100.0 2.0 10.0))
  (`NiagaraComponent.SetNiagaraVariableFloat` _fx "User.Lifetime" (`self.ParticlesLifetime`))
  (`NiagaraComponent.SetNiagaraVariableFloat` _fx "User.ScaleVelo" (`self.ParticlesVelocity`))
  (`NiagaraComponent.SetNiagaraVariableFloat` _fx "User.SpawnRate" (`self.ParticlesSpawnRate`)))

(fn `UserConstructionScript`)