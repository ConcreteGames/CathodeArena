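; BP_Spot is an environment light actor that projects a texture through three spotlights, one each for red, green and blue.
; The construction script gives each spotlight a dynamic light function material from its channel's screen-light instance.
; It then applies the actor's cone angle and intensity to the lights, and its channel texture and time value to the materials.
; BeginPlay, Tick and SwitchOffScreen are empty, so the graphs add no runtime logic.
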(event `self.ReceiveBeginPlay`)

(event `self.ReceiveTick`
  (params (DeltaSeconds :type "Float (single-precision)")))

(event `Constructor`
  (`self.SetSpotOuterConeAngle` (`self.OuterConeAngle`))
  (`self.SetSpotIntensity` (`self.Intensity`))
  (`self.SetSpotChannel` (`self.T_Channel`))
  (`self.SetSpotSpeed` (`self.Time`)))

(event `SwitchOffScreen`)

(fn `SetDynamicLigthMaterial`
  (for _index (range 3)
    (switch `int` _index
      (:`0`
        (bind _returnvalue (`KismetMaterialLibrary.CreateDynamicMaterialInstance` "/Game/CathodeArena/MaterialLibrary/Lights/M_ScreenLight_R_Inst.M_ScreenLight_R_Inst"))
        (bind _output_get (set `self.LightFunctionMatRed` _returnvalue))
        (`LightComponent.SetLightFunctionMaterial` (`self.SpotLightR`) _output_get))
      (:`1`
        (bind _returnvalue_2 (`KismetMaterialLibrary.CreateDynamicMaterialInstance` "/Game/CathodeArena/MaterialLibrary/Lights/M_ScreenLight_G_Inst.M_ScreenLight_G_Inst"))
        (bind _output_get_2 (set `self.LightFunctionMatGreen` _returnvalue_2))
        (`LightComponent.SetLightFunctionMaterial` (`self.SpotLightG`) _output_get_2))
      (:`2`
        (bind _returnvalue_3 (`KismetMaterialLibrary.CreateDynamicMaterialInstance` "/Game/CathodeArena/MaterialLibrary/Lights/M_ScreenLight_B_Inst.M_ScreenLight_B_Inst"))
        (bind _output_get_3 (set `self.LightFunctionMatBlue` _returnvalue_3))
        (`LightComponent.SetLightFunctionMaterial` (`self.SpotLightB`) _output_get_3)))))

(fn `SetSpotChannel`
  (params (Value :type "Texture Object Reference"))
  (`MaterialInstanceDynamic.SetTextureParameterValue` (`self.LightFunctionMatRed`) "Texture" Value)
  (`MaterialInstanceDynamic.SetTextureParameterValue` (`self.LightFunctionMatBlue`) "Texture" Value)
  (`MaterialInstanceDynamic.SetTextureParameterValue` (`self.LightFunctionMatGreen`) "Texture" Value))

(fn `SetSpotIntensity`
  (params (NewIntensity :type "Float (double-precision)"))
  (`LightComponent.SetIntensity` (`self.SpotLightR`) NewIntensity)
  (`LightComponent.SetIntensity` (`self.SpotLightG`) NewIntensity)
  (`LightComponent.SetIntensity` (`self.SpotLightB`) NewIntensity))

(fn `SetSpotOuterConeAngle`
  (params (NewOuterConeAngle :type "Float (double-precision)"))
  (`SpotLightComponent.SetOuterConeAngle` (`self.SpotLightB`) NewOuterConeAngle)
  (`SpotLightComponent.SetOuterConeAngle` (`self.SpotLightG`) NewOuterConeAngle)
  (`SpotLightComponent.SetOuterConeAngle` (`self.SpotLightR`) NewOuterConeAngle))

(fn `SetSpotSpeed`
  (params (Value :type "Float (double-precision)"))
  (`MaterialInstanceDynamic.SetScalarParameterValue` (`self.LightFunctionMatGreen`) "Time" Value)
  (`MaterialInstanceDynamic.SetScalarParameterValue` (`self.LightFunctionMatBlue`) "Time" Value)
  (`MaterialInstanceDynamic.SetScalarParameterValue` (`self.LightFunctionMatRed`) "Time" Value))

(fn `UserConstructionScript`
  (`self.SetDynamicLigthMaterial`)
  (`self.Constructor`))