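; Configurable arena console button that changes colors, fog, gravity, time dilation, particles or player post-process effects according to its EButtonInteractions value.
; Construction script sets category-colored materials, light and label from that enum.
; ActionTriggered, also fired by pinball-ball overlap, animates the press and applies the effect to actors, widgets, world or character.
; Buttons are momentary or FlipFlop toggles, relaying pushed state to ChildInteractableActor via ButtonMessage.
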(event `self.PhysOverlap.OnComponentBeginOverlap`
  (params (OverlappedComponent :type "PrimitiveComponent Object Reference") (OtherActor :type "Actor Object Reference") (OtherComp :type "PrimitiveComponent Object Reference") (OtherBodyIndex :type Integer) (bFromSweep :type Boolean) (SweepResult :type "HitResult Structure (by ref)"))
  (cast `/Game/CathodeArena/Core/PhysicActors/BP_I_PinballBall` OtherActor)
  (`/Game/CathodeArena/Core/Engine/BPI_Actionable.ActionTriggered` false))

(event `PlayButtonAnimation`
  (switch `/Game/CathodeArena/Core/Environment/E_ButtonInteractions` (`self.EButtonInteractions`)
    (:`NewEnumerator6`
      (set `self.IsSimpleTriger` true :!label _label)
      (`self.Push` true)
      (`PrimitiveComponent.SetMaterial` (`self.SM_ButtonPush`) 0 (select `bool` (`self.IsPushed`) :`false` (`self.DMI_NotPushed`) :`true` (`self.DMI_Pushed`) :!type "MaterialInterface Object Reference")))
    (:`NewEnumerator16`
      (goto _label))
    (:`NewEnumerator41`
      (`/Engine/EditorBlueprintResources/StandardMacros.FlipFlop` :!label _label_2
        (:`A`
          (`self.Push` true))
        (:`B`
          (`self.Push` false)))
      (`PrimitiveComponent.SetMaterial` (`self.SM_ButtonPush`) 0 (select `bool` (`self.IsPushed`) :`false` (`self.DMI_NotPushed`) :`true` (`self.DMI_Pushed`) :!type "MaterialInterface Object Reference"))
      (`PrimitiveComponent.SetMaterial` (`self.Sphere`) 0 (select `bool` (`self.IsPushed`) :`false` (`self.DMI_NotPushed`) :`true` (`self.DMI_Pushed`) :!type "MaterialInterface Object Reference")))
    (:`NewEnumerator40`
      (goto _label))
    (:`NewEnumerator7`
      (goto _label))
    (:`NewEnumerator11`
      (goto _label))
    (:`NewEnumerator12`
      (goto _label))
    (:`NewEnumerator13`
      (goto _label))
    (:`NewEnumerator17`
      (goto _label))
    (:`NewEnumerator10`
      (goto _label))
    (:`NewEnumerator14`
      (goto _label))
    (:`NewEnumerator15`
      (goto _label))
    (:`NewEnumerator0`
      (goto _label_2))
    (:`NewEnumerator18`
      (goto _label_2))
    (:`NewEnumerator19`
      (goto _label_2))
    (:`NewEnumerator20`
      (goto _label_2))
    (:`NewEnumerator21`
      (goto _label_2))
    (:`NewEnumerator22`
      (goto _label_2))
    (:`NewEnumerator23`
      (goto _label_2))
    (:`NewEnumerator24`
      (goto _label_2))
    (:`NewEnumerator25`
      (goto _label_2))
    (:`NewEnumerator26`
      (goto _label_2))
    (:`NewEnumerator27`
      (goto _label_2))
    (:`NewEnumerator28`
      (goto _label_2))
    (:`NewEnumerator29`
      (goto _label_2))
    (:`NewEnumerator30`
      (goto _label_2))
    (:`NewEnumerator31`
      (goto _label_2))
    (:`NewEnumerator32`
      (goto _label_2))
    (:`NewEnumerator33`
      (goto _label_2))
    (:`NewEnumerator34`
      (goto _label_2))
    (:`NewEnumerator35`
      (goto _label_2))
    (:`NewEnumerator36`
      (goto _label_2))
    (:`NewEnumerator37`
      (goto _label_2))
    (:`NewEnumerator38`
      (goto _label_2))
    (:`NewEnumerator39`
      (goto _label_2))
    (:`NewEnumerator5`
      (goto _label_2)))
  (`SceneComponent.SetVisibility` (`self.PointLight`) (`self.IsPushed`) false)
  (`TimelineComponent.SetTimelineLength` (`self.PushButton`) 0.1)
  (`Timeline|PushButton` :!via `PlayFromStart`
    (:`Update`
      (`SceneComponent.K2_SetRelativeLocation` (`self.SM_ButtonPush`) (`KismetMathLibrary.MakeVector` 0.0 0.0 (* (`CurveFloat.GetFloatValue` (`self.CRVPushButton`) (`/Game/CathodeArena/Core/Engine/BP_FunctionLibrary.GetTimelinePercentage` (`self.PushButton`))) -30.0)) false false))
    (:`Finished`
      (if (`self.IsSimpleTriger`)
        (`self.Push` false) ; Activate connected child actions
        (`SceneComponent.SetVisibility` (`self.PointLight`) (`self.IsPushed`) false)
        (`PrimitiveComponent.SetMaterial` (`self.SM_ButtonPush`) 0 (select `bool` (`self.IsPushed`) :`false` (`self.DMI_NotPushed`) :`true` (`self.DMI_Pushed`) :!type "MaterialInterface Object Reference"))
        (`PrimitiveComponent.SetMaterial` (`self.Sphere`) 0 (select `bool` (`self.IsPushed`) :`false` (`self.DMI_NotPushed`) :`true` (`self.DMI_Pushed`) :!type "MaterialInterface Object Reference"))))))

(event `OnIsPushed`
  (params (IsPushed :type Boolean))
  (bind _childinteractableactor (`self.ChildInteractableActor`))
  ;[1 1 1] Activate connected child actions
  (if IsPushed
    (message `/Game/CathodeArena/Core/Engine/BPI_Actionable.Button` _childinteractableactor true)
    (else
      (message `/Game/CathodeArena/Core/Engine/BPI_Actionable.Button` _childinteractableactor false))))

(event `/Game/CathodeArena/Core/Engine/BPI_Actionable.ActionTriggered`
  (params (HandIsLeft :type Boolean))
  (bind _returnvalue (`KismetMathLibrary.RandomFloat`))
  (bind _returnvalue_2 (`KismetMathLibrary.RandomFloat`))
  (bind _returnvalue_3 (`KismetMathLibrary.RandomFloat`))
  (bind _returnvalue_4 (`KismetMathLibrary.RandomUnitVector`))
  (bind _minhandcolor (`self.MinHandColor`))
  (bind _maxhandcolor (`self.MaxHandColor`))
  (bind _returnvalue_5 (`KismetMathLibrary.MakeColor` (`KismetMathLibrary.RandomFloatInRange` 0.0 1.0) (`KismetMathLibrary.RandomFloatInRange` 0.0 1.0) (`KismetMathLibrary.RandomFloatInRange` 0.0 1.0)))
  (`self.PlayButtonAnimation`)
  (switch `/Game/CathodeArena/Core/Environment/E_ButtonInteractions` (`self.EButtonInteractions`)
    (:`NewEnumerator6`
      ;[1 1 1] Light Color
      (bind _outactors (`GameplayStatics.GetAllActorsOfClass` "/Game/CathodeArena/Core/Environment/BP_RoofScreen.BP_RoofScreen_C"))
      (`LightComponent.SetLightColor` (`/Game/CathodeArena/Core/Environment/BP_RoofScreen.SpotLight` (`|GetArrayItem` _outactors)) _returnvalue_5 true)
      (bind _outactors_2 (`GameplayStatics.GetAllActorsOfClass` "/Script/Engine.ExponentialHeightFog"))
      (`ExponentialHeightFogComponent.SetFogInscatteringColor` (`ExponentialHeightFog.Component` (`|GetArrayItem` _outactors_2)) _returnvalue_5))
    (:`NewEnumerator16`
      ;[1 1 1] Random Fists Tint
      (bind _foundwidgets (`WidgetBlueprintLibrary.GetAllWidgetsOfClass` "/Game/CathodeArena/Core/HUD/UI_Hands.UI_Hands_C"))
      (`Border.SetContentColorAndOpacity` (`/Game/CathodeArena/Core/HUD/UI_Hands.B_ChangeColor` (`|GetArrayItem` _foundwidgets)) (make `LinearColor` (`KismetMathLibrary.RandomFloatInRange` _minhandcolor _maxhandcolor) (`KismetMathLibrary.RandomFloatInRange` _minhandcolor _maxhandcolor) (`KismetMathLibrary.RandomFloatInRange` _minhandcolor _maxhandcolor) 1.0)))
    (:`NewEnumerator41`
      ;[1 1 1] Props Color
      (`/Engine/EditorBlueprintResources/StandardMacros.FlipFlop`
        (:`A`
          (`/Engine/EditorBlueprintResources/StandardMacros.FlipFlop`
            (:`A`
              (`/Game/CathodeArena/Core/Engine/BP_FunctionLibrary.MeshColor` true (`KismetMathLibrary.RandomFloatInRange` 1.0 50.0) (make `LinearColor` _returnvalue _returnvalue_2 _returnvalue_3 1.0)))
            (:`B`
              (`/Game/CathodeArena/Core/Engine/BP_FunctionLibrary.MeshColor` true 0.0 (make `LinearColor` _returnvalue _returnvalue_2 _returnvalue_3 1.0)))))
        (:`B`
          (`/Game/CathodeArena/Core/Engine/BP_FunctionLibrary.MeshColor` false))))
    (:`NewEnumerator40`
      ;[1 1 1] Fog
      (bind _outactors_3 (`GameplayStatics.GetAllActorsOfClass` "/Script/Engine.ExponentialHeightFog"))
      (bind _component (`ExponentialHeightFog.Component` (`|GetArrayItem` _outactors_3)))
      (`ExponentialHeightFogComponent.SetFogDensity` _component (`KismetMathLibrary.RandomFloatInRange` 1e-06 (select `bool` (<= (`ExponentialHeightFogComponent.FogDensity` _component) 0.1) :`false` 0.001 :`true` 1.0 :!type "Float (single-precision)"))))
    (:`NewEnumerator7`
      ;[1 1 1] GravityForce ++
      (bind _outactors_4 (`GameplayStatics.GetAllActorsOfClass` "/Game/DirectionalGravity/Blueprints/SceneObjects/BP_GravityVolumeBox.BP_GravityVolumeBox_C"))
      (bind _output (`|GetArrayItem` _outactors_4))
      (set `/Game/DirectionalGravity/Blueprints/GravityLogic/BP_GravityVolumeBase.Force` (* (`/Game/DirectionalGravity/Blueprints/GravityLogic/BP_GravityVolumeBase.Force` _output) 1.25) _output))
    (:`NewEnumerator11`
      ;[1 1 1] GravityForce --
      (bind _outactors_5 (`GameplayStatics.GetAllActorsOfClass` "/Game/DirectionalGravity/Blueprints/SceneObjects/BP_GravityVolumeBox.BP_GravityVolumeBox_C"))
      (bind _output_2 (`|GetArrayItem` _outactors_5))
      (set `/Game/DirectionalGravity/Blueprints/GravityLogic/BP_GravityVolumeBase.Force` (* (`/Game/DirectionalGravity/Blueprints/GravityLogic/BP_GravityVolumeBase.Force` _output_2) 0.75) _output_2))
    (:`NewEnumerator12`
      ;[1 1 1] GravityForce Reset
      (bind _outactors_6 (`GameplayStatics.GetAllActorsOfClass` "/Game/DirectionalGravity/Blueprints/SceneObjects/BP_GravityVolumeBox.BP_GravityVolumeBox_C"))
      (set `/Game/DirectionalGravity/Blueprints/GravityLogic/BP_GravityVolumeBase.Force` 3000.0 (`|GetArrayItem` _outactors_6)))
    (:`NewEnumerator13`
      ;[1 1 1] Change Gravity
      (bind _outactors_7 (`GameplayStatics.GetAllActorsOfClass` "/Game/DirectionalGravity/Blueprints/SceneObjects/BP_GravityVolumeBox.BP_GravityVolumeBox_C"))
      (set `/Game/DirectionalGravity/Blueprints/GravityLogic/BP_GravityVolumeBase.LocalDirection` (* (`self.GetActorUpVector`) -1.0) (`|GetArrayItem` _outactors_7)))
    (:`NewEnumerator17`
      ;[1 1 1] TILT
      (bind _outactors_8 (`GameplayStatics.GetAllActorsOfClass` "/Game/CathodeArena/Core/PhysicActors/BP_InteractiveObject.BP_InteractiveObject_C"))
      (for _array_element _outactors_8
        (`PrimitiveComponent.AddImpulse` (`StaticMeshActor.StaticMeshComponent` _array_element) (* _returnvalue_4 4000000.0) "None" false))
      (`PrimitiveComponent.AddImpulse` (`/Game/CathodeArena/Core/Characters/BP_GravityCharacterBase.WalkCollision` (`/Game/CathodeArena/Core/Engine/BP_FunctionLibrary.GetChar`)) (* _returnvalue_4 500000.0) "None" false))
    (:`NewEnumerator10`
      ;[1 1 1] Speed ++
      (`GameplayStatics.SetGlobalTimeDilation` (* (`GameplayStatics.GetGlobalTimeDilation`) 1.25)))
    (:`NewEnumerator14`
      ;[1 1 1] Speed Reset
      (`GameplayStatics.SetGlobalTimeDilation` 1.0))
    (:`NewEnumerator15`
      ;[1 1 1] Speed --
      (`GameplayStatics.SetGlobalTimeDilation` (* (`GameplayStatics.GetGlobalTimeDilation`) 0.75)))
    (:`NewEnumerator0`
      (bind _isa (`/Engine/EditorBlueprintResources/StandardMacros.FlipFlop`)
        (:`A`
          _)
        (:`B`
          _))
      (set `/Game/CathodeArena/Core/Characters/BP_GravityCharacterBase.PP_ChromaticWeight` (select `bool` _isa :`true` (`self.PP_Max`)) (`/Game/CathodeArena/Core/Engine/BP_FunctionLibrary.GetChar`))
      (`/Game/CathodeArena/Core/Characters/BP_GravityCharacterBase.PostProcessesManager` (`/Game/CathodeArena/Core/Engine/BP_FunctionLibrary.GetChar`) :!label _label_3))
    (:`NewEnumerator18`
      (bind _isa_2 (`/Engine/EditorBlueprintResources/StandardMacros.FlipFlop`)
        (:`A`
          _)
        (:`B`
          _))
      (set `/Game/CathodeArena/Core/Characters/BP_GravityCharacterBase.PP_PsycheWeight` (select `bool` _isa_2 :`true` (`self.PP_Max`)) (`/Game/CathodeArena/Core/Engine/BP_FunctionLibrary.GetChar`))
      (goto _label_3))
    (:`NewEnumerator19`
      (bind _isa_3 (`/Engine/EditorBlueprintResources/StandardMacros.FlipFlop`)
        (:`A`
          _)
        (:`B`
          _))
      (set `/Game/CathodeArena/Core/Characters/BP_GravityCharacterBase.PP_PsycheRVB` (select `bool` _isa_3 :`true` (`self.PP_Max`)) (`/Game/CathodeArena/Core/Engine/BP_FunctionLibrary.GetChar`))
      (goto _label_3))
    (:`NewEnumerator20`
      (bind _isa_4 (`/Engine/EditorBlueprintResources/StandardMacros.FlipFlop`)
        (:`A`
          _)
        (:`B`
          _))
      (set `/Game/CathodeArena/Core/Characters/BP_GravityCharacterBase.PP_OutlineWeight` (select `bool` _isa_4 :`true` (`self.PP_Max`)) (`/Game/CathodeArena/Core/Engine/BP_FunctionLibrary.GetChar`))
      (goto _label_3))
    (:`NewEnumerator21`
      (bind _isa_5 (`/Engine/EditorBlueprintResources/StandardMacros.FlipFlop`)
        (:`A`
          _)
        (:`B`
          _))
      (set `/Game/CathodeArena/Core/Characters/BP_GravityCharacterBase.PP_Outline2ColorsWeight` (select `bool` _isa_5 :`true` (`self.PP_Max`)) (`/Game/CathodeArena/Core/Engine/BP_FunctionLibrary.GetChar`))
      (goto _label_3))
    (:`NewEnumerator22`
      (bind _isa_6 (`/Engine/EditorBlueprintResources/StandardMacros.FlipFlop`)
        (:`A`
          _)
        (:`B`
          _))
      (set `/Game/CathodeArena/Core/Characters/BP_GravityCharacterBase.PP_TVLines` (select `bool` _isa_6 :`true` (`self.PP_Max`)) (`/Game/CathodeArena/Core/Engine/BP_FunctionLibrary.GetChar`))
      (goto _label_3))
    (:`NewEnumerator23`
      (bind _isa_7 (`/Engine/EditorBlueprintResources/StandardMacros.FlipFlop`)
        (:`A`
          _)
        (:`B`
          _))
      (set `/Game/CathodeArena/Core/Characters/BP_GravityCharacterBase.PP_ArcadeScanlines` (select `bool` _isa_7 :`true` (`self.PP_Max`)) (`/Game/CathodeArena/Core/Engine/BP_FunctionLibrary.GetChar`))
      (goto _label_3))
    (:`NewEnumerator24`
      (bind _isa_8 (`/Engine/EditorBlueprintResources/StandardMacros.FlipFlop`)
        (:`A`
          _)
        (:`B`
          _))
      (set `/Game/CathodeArena/Core/Characters/BP_GravityCharacterBase.PP_ASCII` (select `bool` _isa_8 :`true` (`self.PP_Max`)) (`/Game/CathodeArena/Core/Engine/BP_FunctionLibrary.GetChar`))
      (goto _label_3))
    (:`NewEnumerator25`
      (bind _isa_9 (`/Engine/EditorBlueprintResources/StandardMacros.FlipFlop`)
        (:`A`
          _)
        (:`B`
          _))
      (set `/Game/CathodeArena/Core/Characters/BP_GravityCharacterBase.PP_Broken Glass` (select `bool` _isa_9 :`true` (`self.PP_Max`)) (`/Game/CathodeArena/Core/Engine/BP_FunctionLibrary.GetChar`))
      (goto _label_3))
    (:`NewEnumerator26`
      (bind _isa_10 (`/Engine/EditorBlueprintResources/StandardMacros.FlipFlop`)
        (:`A`
          _)
        (:`B`
          _))
      (set `/Game/CathodeArena/Core/Characters/BP_GravityCharacterBase.PP_Bump` (select `bool` _isa_10 :`true` (`self.PP_Max`)) (`/Game/CathodeArena/Core/Engine/BP_FunctionLibrary.GetChar`))
      (goto _label_3))
    (:`NewEnumerator27`
      (bind _isa_11 (`/Engine/EditorBlueprintResources/StandardMacros.FlipFlop`)
        (:`A`
          _)
        (:`B`
          _))
      (set `/Game/CathodeArena/Core/Characters/BP_GravityCharacterBase.PP_Chromatic Blur` (select `bool` _isa_11 :`true` (`self.PP_Max`)) (`/Game/CathodeArena/Core/Engine/BP_FunctionLibrary.GetChar`))
      (goto _label_3))
    (:`NewEnumerator28`
      (bind _isa_12 (`/Engine/EditorBlueprintResources/StandardMacros.FlipFlop`)
        (:`A`
          _)
        (:`B`
          _))
      (set `/Game/CathodeArena/Core/Characters/BP_GravityCharacterBase.PP_Difference` (select `bool` _isa_12 :`true` (`self.PP_Max`)) (`/Game/CathodeArena/Core/Engine/BP_FunctionLibrary.GetChar`))
      (goto _label_3))
    (:`NewEnumerator29`
      (bind _isa_13 (`/Engine/EditorBlueprintResources/StandardMacros.FlipFlop`)
        (:`A`
          _)
        (:`B`
          _))
      (set `/Game/CathodeArena/Core/Characters/BP_GravityCharacterBase.PP_Dithering` (select `bool` _isa_13 :`true` (`self.PP_Max`)) (`/Game/CathodeArena/Core/Engine/BP_FunctionLibrary.GetChar`))
      (goto _label_3))
    (:`NewEnumerator30`
      (bind _isa_14 (`/Engine/EditorBlueprintResources/StandardMacros.FlipFlop`)
        (:`A`
          _)
        (:`B`
          _))
      (set `/Game/CathodeArena/Core/Characters/BP_GravityCharacterBase.PP_Dithering Glitch` (select `bool` _isa_14 :`true` (`self.PP_Max`)) (`/Game/CathodeArena/Core/Engine/BP_FunctionLibrary.GetChar`))
      (goto _label_3))
    (:`NewEnumerator31`
      (bind _isa_15 (`/Engine/EditorBlueprintResources/StandardMacros.FlipFlop`)
        (:`A`
          _)
        (:`B`
          _))
      (set `/Game/CathodeArena/Core/Characters/BP_GravityCharacterBase.PP_Frozen Glass` (select `bool` _isa_15 :`true` (`self.PP_Max`)) (`/Game/CathodeArena/Core/Engine/BP_FunctionLibrary.GetChar`))
      (goto _label_3))
    (:`NewEnumerator32`
      (bind _isa_16 (`/Engine/EditorBlueprintResources/StandardMacros.FlipFlop`)
        (:`A`
          _)
        (:`B`
          _))
      (set `/Game/CathodeArena/Core/Characters/BP_GravityCharacterBase.PP_Glitch` (select `bool` _isa_16 :`true` (`self.PP_Max`)) (`/Game/CathodeArena/Core/Engine/BP_FunctionLibrary.GetChar`))
      (goto _label_3))
    (:`NewEnumerator33`
      (bind _isa_17 (`/Engine/EditorBlueprintResources/StandardMacros.FlipFlop`)
        (:`A`
          _)
        (:`B`
          _))
      (set `/Game/CathodeArena/Core/Characters/BP_GravityCharacterBase.PP_Lens Distortion` (select `bool` _isa_17 :`true` (`self.PP_Max`)) (`/Game/CathodeArena/Core/Engine/BP_FunctionLibrary.GetChar`))
      (goto _label_3))
    (:`NewEnumerator34`
      (bind _isa_18 (`/Engine/EditorBlueprintResources/StandardMacros.FlipFlop`)
        (:`A`
          _)
        (:`B`
          _))
      (set `/Game/CathodeArena/Core/Characters/BP_GravityCharacterBase.PP_Posterize Pixelate` (select `bool` _isa_18 :`true` (`self.PP_Max`)) (`/Game/CathodeArena/Core/Engine/BP_FunctionLibrary.GetChar`))
      (goto _label_3))
    (:`NewEnumerator35`
      (bind _isa_19 (`/Engine/EditorBlueprintResources/StandardMacros.FlipFlop`)
        (:`A`
          _)
        (:`B`
          _))
      (set `/Game/CathodeArena/Core/Characters/BP_GravityCharacterBase.PP_Pulse Force` (select `bool` _isa_19 :`true` (`self.PP_Max`)) (`/Game/CathodeArena/Core/Engine/BP_FunctionLibrary.GetChar`))
      (goto _label_3))
    (:`NewEnumerator36`
      (bind _isa_20 (`/Engine/EditorBlueprintResources/StandardMacros.FlipFlop`)
        (:`A`
          _)
        (:`B`
          _))
      (set `/Game/CathodeArena/Core/Characters/BP_GravityCharacterBase.PP_Pulse Wallhack` (select `bool` _isa_20 :`true` (`self.PP_Max`)) (`/Game/CathodeArena/Core/Engine/BP_FunctionLibrary.GetChar`))
      (goto _label_3))
    (:`NewEnumerator37`
      (bind _isa_21 (`/Engine/EditorBlueprintResources/StandardMacros.FlipFlop`)
        (:`A`
          _)
        (:`B`
          _))
      (set `/Game/CathodeArena/Core/Characters/BP_GravityCharacterBase.PP_Sharpen` (select `bool` _isa_21 :`true` (`self.PP_Max`)) (`/Game/CathodeArena/Core/Engine/BP_FunctionLibrary.GetChar`))
      (goto _label_3))
    (:`NewEnumerator38`
      (bind _isa_22 (`/Engine/EditorBlueprintResources/StandardMacros.FlipFlop`)
        (:`A`
          _)
        (:`B`
          _))
      (set `/Game/CathodeArena/Core/Characters/BP_GravityCharacterBase.PP_TV Cathode Ray Tube` (select `bool` _isa_22 :`true` (`self.PP_Max`)) (`/Game/CathodeArena/Core/Engine/BP_FunctionLibrary.GetChar`))
      (goto _label_3))
    (:`NewEnumerator39`
      (bind _isa_23 (`/Engine/EditorBlueprintResources/StandardMacros.FlipFlop`)
        (:`A`
          _)
        (:`B`
          _))
      (set `/Game/CathodeArena/Core/Characters/BP_GravityCharacterBase.PP_Underwater` (select `bool` _isa_23 :`true` (`self.PP_Max`)) (`/Game/CathodeArena/Core/Engine/BP_FunctionLibrary.GetChar`))
      (goto _label_3))
    (:`NewEnumerator5`
      ;[1 1 1] Particles
      (bind _outactors_9 (`GameplayStatics.GetAllActorsOfClass` "/Game/CathodeArena/Core/Environment/BP_ParticleManager.BP_ParticleManager_C"))
      (`/Game/CathodeArena/Core/Environment/BP_ParticleManager.TriggerParticles` (`|GetArrayItem` _outactors_9)))))

(fn `Push`
  (params (IsPushed :type Boolean))
  (bind _output_get (set `self.IsPushed` IsPushed))
  (`self.OnIsPushed` _output_get))

(fn `UserConstructionScript`
  (bind _texte (`self.Texte`))
  (bind _returnvalue (select `/Game/CathodeArena/Core/Environment/E_ButtonInteractions` (`self.EButtonInteractions`) :`NewEnumerator6` (struct :`R` 1.0 :`G` 1.0 :`A` 1.0) :`NewEnumerator16` (struct :`R` 1.0 :`G` 1.0 :`A` 1.0) :`NewEnumerator41` (struct :`R` 1.0 :`G` 1.0 :`A` 1.0) :`NewEnumerator40` (struct :`R` 1.0 :`G` 1.0 :`A` 1.0) :`NewEnumerator7` (struct :`R` 1.0 :`A` 1.0) :`NewEnumerator11` (struct :`R` 1.0 :`A` 1.0) :`NewEnumerator12` (struct :`R` 1.0 :`A` 1.0) :`NewEnumerator13` (struct :`R` 1.0 :`A` 1.0) :`NewEnumerator17` (struct :`R` 1.0 :`A` 1.0) :`NewEnumerator10` (struct :`R` 1.0 :`B` 1.0 :`A` 1.0) :`NewEnumerator14` (struct :`R` 1.0 :`B` 1.0 :`A` 1.0) :`NewEnumerator15` (struct :`R` 1.0 :`B` 1.0 :`A` 1.0) :`NewEnumerator0` (struct :`G` 1.0 :`B` 1.0 :`A` 1.0) :`NewEnumerator18` (struct :`G` 1.0 :`B` 1.0 :`A` 1.0) :`NewEnumerator19` (struct :`G` 1.0 :`B` 1.0 :`A` 1.0) :`NewEnumerator20` (struct :`G` 1.0 :`B` 1.0 :`A` 1.0) :`NewEnumerator21` (struct :`G` 1.0 :`B` 1.0 :`A` 1.0) :`NewEnumerator22` (struct :`G` 1.0 :`B` 1.0 :`A` 1.0) :`NewEnumerator23` (struct :`G` 1.0 :`B` 1.0 :`A` 1.0) :`NewEnumerator24` (struct :`G` 1.0 :`B` 1.0 :`A` 1.0) :`NewEnumerator25` (struct :`G` 1.0 :`B` 1.0 :`A` 1.0) :`NewEnumerator26` (struct :`G` 1.0 :`B` 1.0 :`A` 1.0) :`NewEnumerator27` (struct :`G` 1.0 :`B` 1.0 :`A` 1.0) :`NewEnumerator28` (struct :`G` 1.0 :`B` 1.0 :`A` 1.0) :`NewEnumerator29` (struct :`G` 1.0 :`B` 1.0 :`A` 1.0) :`NewEnumerator30` (struct :`G` 1.0 :`B` 1.0 :`A` 1.0) :`NewEnumerator31` (struct :`G` 1.0 :`B` 1.0 :`A` 1.0) :`NewEnumerator32` (struct :`G` 1.0 :`B` 1.0 :`A` 1.0) :`NewEnumerator33` (struct :`G` 1.0 :`B` 1.0 :`A` 1.0) :`NewEnumerator34` (struct :`G` 1.0 :`B` 1.0 :`A` 1.0) :`NewEnumerator35` (struct :`G` 1.0 :`B` 1.0 :`A` 1.0) :`NewEnumerator36` (struct :`G` 1.0 :`B` 1.0 :`A` 1.0) :`NewEnumerator37` (struct :`G` 1.0 :`B` 1.0 :`A` 1.0) :`NewEnumerator38` (struct :`G` 1.0 :`B` 1.0 :`A` 1.0) :`NewEnumerator39` (struct :`G` 1.0 :`B` 1.0 :`A` 1.0) :`NewEnumerator5` (struct :`G` 1.0 :`A` 1.0) :!type "LinearColor Structure"))
  (bind _returnvalue_2 (* _returnvalue 40.0))
  (bind _returnvalue_3 (`PrimitiveComponent.CreateDynamicMaterialInstance` (`self.SM_ButtonPush`) 0 "/Game/CathodeArena/Art/Props/Button/M_ButtonNotPushed_Inst.M_ButtonNotPushed_Inst" "None"))
  (bind _output_get (set `self.DMI_NotPushed` _returnvalue_3))
  (`MaterialInstanceDynamic.SetVectorParameterValue` _output_get "Base Color" (* _returnvalue 0.5))
  (`PrimitiveComponent.SetMaterial` (`self.Sphere`) 0 (`self.DMI_NotPushed`))
  (bind _returnvalue_4 (`KismetMaterialLibrary.CreateDynamicMaterialInstance` (`self.PushedMaterial`) "/Game/CathodeArena/Art/Props/Button/M_ButtonPushed.M_ButtonPushed"))
  (bind _output_get_2 (set `self.DMI_Pushed` _returnvalue_4))
  (`MaterialInstanceDynamic.SetVectorParameterValue` _output_get_2 "Base Color" _returnvalue_2)
  (`LightComponent.SetLightColor` (`self.PointLight`) _returnvalue_2 true)
  (`TextRenderComponent.K2_SetText` (`self.TextRender`) (`KismetTextLibrary.Conv_StringToText` (select `bool` (`KismetStringLibrary.EqualEqual_StrStr` _texte "BUTTON") :`false` _texte :`true` (select `/Game/CathodeArena/Core/Environment/E_ButtonInteractions` (`self.EButtonInteractions`) :`NewEnumerator6` "Light Color" :`NewEnumerator16` "Hands Color" :`NewEnumerator41` "Props Color" :`NewEnumerator40` "Fog" :`NewEnumerator7` "More Gravity" :`NewEnumerator11` "Less Gravity" :`NewEnumerator12` "Reset Gravity" :`NewEnumerator13` "?" :`NewEnumerator17` "TILT" :`NewEnumerator10` "Faster!" :`NewEnumerator14` "Normal Speed" :`NewEnumerator15` "Slowdown..." :`NewEnumerator0` "Chromatic \nAberation" :`NewEnumerator18` "Psyche \nCel Shading" :`NewEnumerator19` "Psyche \nToon RVB" :`NewEnumerator20` "Black \nOutline" :`NewEnumerator21` "Digital \nOutline" :`NewEnumerator22` "TV Lines" :`NewEnumerator23` "Arcade \nScanlines" :`NewEnumerator24` "ASCII" :`NewEnumerator25` "Broken \nGlass" :`NewEnumerator26` "Bump" :`NewEnumerator27` "Chromatic Blur" :`NewEnumerator28` "Difference" :`NewEnumerator29` "Dithering" :`NewEnumerator30` "Dithering Glitch" :`NewEnumerator31` "Frozen Glass" :`NewEnumerator32` "Glitch" :`NewEnumerator33` "Lens \nDistortion" :`NewEnumerator34` "Posterize \nPixelate" :`NewEnumerator35` "Pulse Force" :`NewEnumerator36` "Pulse \nWallhack" :`NewEnumerator37` "Hard \nSharpen" :`NewEnumerator38` "TV Cathode \nRay Tube" :`NewEnumerator39` "Underwater" :`NewEnumerator5` "NEED Particles!")))))