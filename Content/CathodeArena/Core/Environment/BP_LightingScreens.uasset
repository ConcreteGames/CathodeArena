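; BP_LightingScreens is an environment screen that pairs a textured plane with red, green and blue lights, apparently to mimic light cast by the display.
; Its construction script sizes the plane and creates a dynamic screen material fed with a texture and time value.
; It also sets rect light intensity, radius and light-function scale from ScreenScale, and assigns per-channel light function materials to spot lights.
; The event graph is empty.
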(event `self.ReceiveBeginPlay`)

(event `self.ReceiveTick`
  (params (DeltaSeconds :type "Float (single-precision)")))

(fn `UserConstructionScript`
  (bind _screenscale_x (`KismetMathLibrary.BreakVector` (`self.ScreenScale`)))
  (bind _midscreen (`self.MidScreen`))
  (bind _returnvalue (* _screenscale_x 100.0))
  (`SceneComponent.SetWorldScale3D` (`self.Plane`) (`self.ScreenScale`))
  (`LightComponent.SetLightFunctionScale` (`self.RectLightR`) (`KismetMathLibrary.MakeVector` _returnvalue _returnvalue _returnvalue))
  (`LightComponent.SetLightFunctionScale` (`self.RectLightG`) (`KismetMathLibrary.MakeVector` _returnvalue _returnvalue _returnvalue))
  (`LightComponent.SetLightFunctionScale` (`self.RectLightB`) (`KismetMathLibrary.MakeVector` _returnvalue _returnvalue _returnvalue))
  (`LocalLightComponent.SetAttenuationRadius` (`self.RectLightB`) (`self.AttenuationRadius`))
  (`LocalLightComponent.SetAttenuationRadius` (`self.RectLightG`) (`self.AttenuationRadius`))
  (`LocalLightComponent.SetAttenuationRadius` (`self.RectLightR`) (`self.AttenuationRadius`))
  (`LightComponent.SetIntensity` (`self.RectLightG`) (`self.Intensity`))
  (`LightComponent.SetIntensity` (`self.RectLightR`) (`self.Intensity`))
  (`LightComponent.SetIntensity` (`self.RectLightB`) (`self.Intensity`))
  (bind _returnvalue_2 (`PrimitiveComponent.CreateDynamicMaterialInstance` (`self.Plane`) 0 "/Game/CathodeArena/MaterialLibrary/Screens/M_Screen_Inst.M_Screen_Inst" "None"))
  (set `self.MidScreen` _returnvalue_2)
  (`LightComponent.SetLightFunctionMaterial` (`self.SpotLightR`) (`self.LFMR`))
  (`LightComponent.SetLightFunctionMaterial` (`self.SpotLightG`) (`self.LFMG`))
  (`LightComponent.SetLightFunctionMaterial` (`self.SpotLightB`) (`self.LFMB`))
  (`MaterialInstanceDynamic.SetTextureParameterValue` _midscreen "Texture" (`self.MidTexture`))
  (`MaterialInstanceDynamic.SetScalarParameterValue` _midscreen "Time" (`self.Time`)))