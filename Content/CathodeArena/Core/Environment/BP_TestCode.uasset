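; BP_TestCode is a scratch test Blueprint in the CathodeArena environment folder.
; On BeginPlay it waits briefly, logs a message, then starts a looping timer that logs a test message every second.
; Unconnected snippets, which never run, hold debug tweaks for the first BP_GravityVolumeBox's force and direction and for global time dilation.
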(event `test`
  (`/Game/CathodeArena/Core/Engine/BP_FunctionLibrary.LogErer` "test"))

(event `self.ReceiveBeginPlay`
  (`KismetSystemLibrary.Delay` 2.0)
  (`/Game/CathodeArena/Core/Engine/BP_FunctionLibrary.LogErer` "play test code")
  (`KismetSystemLibrary.K2_SetTimerDelegate` (delegate `test`) 1.0 true))

(fn `UserConstructionScript`)