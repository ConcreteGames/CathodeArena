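; BP_Buttons is a pushable arena button that, when triggered, sends its pressed state to a linked ChildInteractableActor through ButtonMessage.
; An EButtonInteractions switch makes each type either a FlipFlop toggle or a momentary trigger that releases when the push animation finishes.
; A curve-driven timeline moves the mesh, while dynamic materials and a point light, tinted from BaseColor, show the pushed state.
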(event `self.ReceiveBeginPlay`
  (bind _sm_buttonpush (`self.SM_ButtonPush`))
  (bind _basematerial (`self.BaseMaterial`))
  (bind _returnvalue (`KismetMaterialLibrary.CreateDynamicMaterialInstance` (`self.PushedMaterial`) "/Game/CathodeArena/Art/Props/Button/M_ButtonPushed.M_ButtonPushed"))
  (bind _output_get (set `self.MidPushed` _returnvalue))
  (`MaterialInstanceDynamic.SetVectorParameterValue` _output_get "Base Color" (`self.PushedColor`))
  (`PrimitiveComponent.SetMaterial` _sm_buttonpush 0 _basematerial)
  (bind _returnvalue_2 (`PrimitiveComponent.CreateDynamicMaterialInstance` _sm_buttonpush 0 _basematerial "None"))
  (`MaterialInstanceDynamic.SetVectorParameterValue` _returnvalue_2 "Base Color" (`self.BaseColor`))
  (bind _outactors (`GameplayStatics.GetAllActorsWithInterface` "/Game/CathodeArena/Core/Engine/BPI_Actionable.BPI_Actionable_C"))
  (for _array_element _outactors
    (if (== _array_element (`self.ChildInteractableActor`))
      _)))

(event `/Game/CathodeArena/Core/Engine/BPI_Actionable.ActionTriggered`
  ;[1 1 1] Hit Button
  (switch `/Game/CathodeArena/Core/Environment/E_ButtonInteractions` (`self.EButtonInteractions`)
    (:`NewEnumerator0`
      (`/Engine/EditorBlueprintResources/StandardMacros.FlipFlop` :!label _label
        (:`A`
          (`self.Push` true))
        (:`B`
          (`self.Push` false)))
      (`PrimitiveComponent.SetMaterial` (`self.SM_ButtonPush`) 0 (select `bool` (`self.IsPushed`) :`false` (`self.MidBase`) :`true` (`self.MidPushed`) :!type "MaterialInterface Object Reference")))
    (:`NewEnumerator1`
      (goto _label))
    (:`NewEnumerator5`
      (set `self.IsSimpleTriger` true :!label _label_2)
      (`self.Push` true)
      (`PrimitiveComponent.SetMaterial` (`self.SM_ButtonPush`) 0 (select `bool` (`self.IsPushed`) :`false` (`self.MidBase`) :`true` (`self.MidPushed`) :!type "MaterialInterface Object Reference")))
    (:`NewEnumerator6`
      (goto _label_2))
    (:`NewEnumerator7`
      (goto _label_2))
    (:`NewEnumerator8`
      (goto _label_2))
    (:`NewEnumerator9`
      (goto _label_2))
    (:`NewEnumerator10`
      (goto _label)))
  (`SceneComponent.SetVisibility` (`self.PointLight`) (`self.IsPushed`) false)
  (`TimelineComponent.SetTimelineLength` (`self.PushButton`) 0.1)
  (`Timeline|PushButton` :!via `PlayFromStart`
    (:`Update`
      (`SceneComponent.K2_SetRelativeLocation` (`self.SM_ButtonPush`) (`KismetMathLibrary.MakeVector` 0.0 0.0 (* (`CurveFloat.GetFloatValue` (`self.CRVPushButton`) (`/Game/CathodeArena/Core/Engine/BP_FunctionLibrary.GetTimelinePercentage` (`self.PushButton`))) -30.0)) false false))
    (:`Finished`
      (if (`self.IsSimpleTriger`)
        (`self.Push` false)
        (`SceneComponent.SetVisibility` (`self.PointLight`) (`self.IsPushed`) false)
        (`PrimitiveComponent.SetMaterial` (`self.SM_ButtonPush`) 0 (select `bool` (`self.IsPushed`) :`false` (`self.MidBase`) :`true` (`self.MidPushed`) :!type "MaterialInterface Object Reference"))))))

(event `OnIsPushed`
  (params (IsPushed :type Boolean))
  (bind _childinteractableactor (`self.ChildInteractableActor`))
  ;[1 1 1] On is Pushed
  (if IsPushed
    (message `/Game/CathodeArena/Core/Engine/BPI_Actionable.Button` _childinteractableactor true)
    (else
      (message `/Game/CathodeArena/Core/Engine/BPI_Actionable.Button` _childinteractableactor false))))

(fn `Push`
  (params (IsPushed :type Boolean))
  (bind _output_get (set `self.IsPushed` IsPushed))
  (`self.OnIsPushed` _output_get))

(fn `UserConstructionScript`
  (bind _sm_buttonpush (`self.SM_ButtonPush`))
  (bind _basecolor (`self.BaseColor`))
  (bind _basematerial (`self.BaseMaterial`))
  (`PrimitiveComponent.SetMaterial` _sm_buttonpush 0 _basematerial)
  (bind _returnvalue (`PrimitiveComponent.CreateDynamicMaterialInstance` _sm_buttonpush 0 _basematerial "None"))
  (bind _output_get (set `self.MidBase` _returnvalue))
  (`MaterialInstanceDynamic.SetVectorParameterValue` _output_get "Base Color" _basecolor)
  (set `self.PushedColor` (* _basecolor 2.0))
  (`LightComponent.SetLightColor` (`self.PointLight`) (`self.PushedColor`) true))