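; BP_ParticleManager switches arena particle effects on and off by name: electric storm, confetti and a Niagara light cylinder.
; On BeginPlay it caches all destructibles, button consoles and the roof screen.
; The storm spawns multiple electricity systems with beam endpoints at random cached console or destructible locations, destroying them when switched off.
; The cylinder gets random life and emissive values plus the roof screen's color, which CylinderColor can update live.
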(event `self.ReceiveBeginPlay`
  (bind _outactors (`GameplayStatics.GetAllActorsOfClass` "/Game/CathodeArena/Core/Destructibles/BP_DestructibleParent.BP_DestructibleParent_C"))
  (for _array_element _outactors
    (`KismetArrayLibrary.Array_AddUnique` (`self.Destructibles`) _array_element))
  (bind _outactors_2 (`GameplayStatics.GetAllActorsOfClass` "/Game/CathodeArena/Core/Environment/BP_ButtonsConsole.BP_ButtonsConsole_C"))
  (for _array_element_2 _outactors_2
    (`KismetArrayLibrary.Array_AddUnique` (`self.Consoles`) _array_element_2))
  (bind _outactors_3 (`GameplayStatics.GetAllActorsOfClass` "/Game/CathodeArena/Core/Environment/BP_RoofScreen.BP_RoofScreen_C"))
  (set `self.RefRoof` (`|GetArrayItem` _outactors_3)))

(event `TriggerParticles`
  (params (Activate :type Boolean) (Name :type Name))
  (bind _confettis (`self.Confettis`))
  (switch `name` Name
    (:`Electric`
      (if Activate
        (`ActorComponent.Activate` (`self.ElectricBeam`) false)
        (`self.ElectricBeamVectors`)
        (else
          (for _array_element (`self.SpawnedElectricity`)
            (`ActorComponent.K2_DestroyComponent` _array_element))
          (`KismetArrayLibrary.Array_Clear` (`self.SpawnedElectricity`)))))
    (:`Confettis`
      (if Activate
        (`ActorComponent.Activate` _confettis false)
        (else
          (`ActorComponent.Deactivate` _confettis))))
    (:`Grid`
      (if Activate
        (bind _returnvalue (`NiagaraFunctionLibrary.SpawnSystemAtLocation` "/Game/CathodeArena/Art/Particles/Partycles/N_LightCylinder_E_System.N_LightCylinder_E_System"))
        (set `self.CylinderParticles` _returnvalue)
        (`NiagaraComponent.SetNiagaraVariableFloat` _returnvalue "User.Life" (`KismetMathLibrary.RandomFloatInRange` 5.0 10.0))
        (`NiagaraComponent.SetNiagaraVariableFloat` _returnvalue "User.Emissive" (`KismetMathLibrary.RandomFloatInRange` 2.0 10.0))
        (`NiagaraComponent.SetNiagaraVariableLinearColor` _returnvalue "User.Color" (`/Game/CathodeArena/Core/Environment/BP_RoofScreen.LigthColor` (`self.RefRoof`)))
        (`ActorComponent.Activate` _returnvalue false)
        (else
          (`ActorComponent.Deactivate` (`self.CylinderParticles`)))))))

(event `CylinderColor`
  (params (Color :type "LinearColor Structure (by ref)"))
  (bind _cylinderparticles (`self.CylinderParticles`))
  (`/Engine/EditorBlueprintResources/StandardMacros.IsValid` _cylinderparticles
    (:`Is Valid`
      (`NiagaraComponent.SetNiagaraVariableLinearColor` _cylinderparticles "User.Color" Color))))

(fn `ElectricBeamVectors`
  (for _ (range (+ (`self.MaxStorm`) 1))
    (bind _returnvalue (`NiagaraFunctionLibrary.SpawnSystemAttached` "/Game/CathodeArena/Art/Particles/Partycles/N_Electricity_S.N_Electricity_S" (`self.ElectricBeam`) "None" (`self.GetActorRandomLocation`) (struct) "KeepRelativeOffset" true))
    (`KismetArrayLibrary.Array_AddUnique` (`self.SpawnedElectricity`) _returnvalue)
    (`NiagaraComponent.SetNiagaraVariableVec3` _returnvalue "User.BeamStart" (`self.GetActorRandomLocation`))
    (`NiagaraComponent.SetNiagaraVariableVec3` _returnvalue "User.BeamEnd" (`self.GetActorRandomLocation`))))

(fn `GetActorRandomLocation`
  (returns (ReturnValue :type "Vector Structure"))
  (bind _destructibles (`self.Destructibles`))
  (bind _consoles (`self.Consoles`))
  (return (select `bool` (`KismetMathLibrary.RandomBool`) :`false` (`self.K2_GetActorLocation` (`|GetArrayItem` _destructibles (`KismetMathLibrary.RandomInteger` (`KismetArrayLibrary.Array_Length` _destructibles)))) :`true` (`self.K2_GetActorLocation` (`|GetArrayItem` _consoles (`KismetMathLibrary.RandomInteger` (`KismetArrayLibrary.Array_Length` _consoles)))))))

(fn `RandomVector`
  (returns (Vector :type "Vector Structure"))
  (return (`KismetMathLibrary.MakeVector` (`KismetMathLibrary.RandomFloatInRange` -2000.0 2000.0) (`KismetMathLibrary.RandomFloatInRange` -2000.0 2000.0) (`KismetMathLibrary.RandomFloatInRange` 0.0 5000.0))))

(fn `UserConstructionScript`)