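; Adaptive music controller that plays the Music component and drives its MusicMain and MusicSub section parameters from timeline beat callbacks.
; MultiGate-filtered beat counters raise the sub part every 8 bars and change the main part every 32, with a 6-bar exit from part 0.
; Main parts advance in order until reaching 6, then switch to random increments.
; Reset zeroes both parts and pulses a Reset parameter, while MusicPart is an empty stub.
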(event `MusicPart`
  (params (Bordel :type Integer)))

(event `CalculateParts`
  (bind _mainbars (`self.MainBars`))
  (bind _mainbars_2 (`self.MainBars`))
  (bind _mainparts (`self.MainParts`))
  (bind _returnvalue (>= _mainparts 6.0))
  (`|MultiGate` false true
    (:`Out 0`
      (set `self.MainBars` (+ _mainbars_2 1))
      (if (and (== (mod _mainbars_2 32) 0) (!= _mainbars_2 0))
        (if (not (`self.Randomize`))
          (set `self.Randomize` _returnvalue)
          (set `self.MainParts` (select `bool` (`self.Randomize`) :`false` (select `bool` _returnvalue :`false` (+ _mainparts 1.0) :`true` 1.0) :`true` (select `bool` false :`false` (+ (`self.MainParts`) (`KismetMathLibrary.Conv_IntToDouble` (`KismetMathLibrary.FFloor` (`KismetMathLibrary.RandomFloatInRange` 1.0 6.0)))) :`true` 1.0)) :!label _label))
        (`FMODAudioComponent.SetParameter` (`self.Music`) "MusicMain" (`self.MainParts`))
        (set `self.SubParts` 0.0)
        (`FMODAudioComponent.SetParameter` (`self.Music`) "MusicSub" (`self.SubParts`))
        (else
          (bind _returnvalue_2 (`FMODAudioComponent.GetParameter` (`self.Music`) "MusicMain"))
          (if (== _returnvalue_2 0.0)
            (if (and (== (mod _mainbars 6) 0) (!= _mainbars 0))
              (goto _label))))))))

(event `self.ReceiveBeginPlay`
  (`FMODAudioComponent.Play` (`self.Music`)))

(event `self.Music.OnTimelineBeat`
  (params (Bar :type Integer) (Beat :type Integer) (Position :type Integer) (Tempo :type "Float (single-precision)") (TimeSignatureUpper :type Integer) (TimeSignatureLower :type Integer))
  (`self.CalculateParts`)
  (`|MultiGate` false true
    (:`Out 0`
      (bind _output_get (set `self.Bars` (+ (`self.Bars`) 1)))
      (if (and (== (mod _output_get 8) 0) (!= (`self.Bars`) 0))
        (set `self.SubParts` (+ (`self.SubParts`) 1.0))
        (`FMODAudioComponent.SetParameter` (`self.Music`) "MusicSub" (`self.SubParts`))))))

(event `Reset`
  (`FMODAudioComponent.SetParameter` (`self.Music`) "MusicSub" 0.0)
  (bind _output_get (set `self.MainParts` 0.0))
  (`FMODAudioComponent.SetParameter` (`self.Music`) "MusicMain" _output_get)
  (`FMODAudioComponent.SetParameter` (`self.Music`) "Reset" 1.0)
  (`KismetSystemLibrary.Delay` 2.0)
  (`FMODAudioComponent.SetParameter` (`self.Music`) "Reset" 0.0))

(fn `UserConstructionScript`)