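; Configurable physics prop that takes its static mesh from a variable in the construction script and overrides its mass on BeginPlay.
; When the hit result's component carries the "Arm" tag, it plays a 2D impact sound.
; A gate closes briefly after each sound to throttle repeats from continuous contact.
; Damage received is only logged.
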(event `self.ReceiveBeginPlay`
  (`PrimitiveComponent.SetMassOverrideInKg` (`self.BaseMesh`) "None" (`self.MassKg`) true))

(event `self.BaseMesh.OnComponentHit`
  (params (HitComponent :type "PrimitiveComponent Object Reference") (OtherActor :type "Actor Object Reference") (OtherComp :type "PrimitiveComponent Object Reference") (NormalImpulse :type "Vector Structure") (Hit :type "HitResult Structure (by ref)"))
  ;[1 1 1] Sound
  (`/Engine/EditorBlueprintResources/StandardMacros.Gate` false :!label _label
    (:`Exit`
      (if (`ActorComponent.ComponentHasTag` Hit_HitComponent "Arm")
        (`FMODBlueprintStatics.PlayEvent2D` "/Game/FMOD/Events/Gameplay/ENV_Hit.ENV_Hit")
        (`self.CloseSoundGate`)
        (`KismetSystemLibrary.Delay` 0.2)
        (`self.OpenSoundGate`)))))

(event `OpenSoundGate`
  ;[1 1 1] Sound
  (goto _label :!via `Open`))

(event `CloseSoundGate`
  ;[1 1 1] Sound
  (goto _label :!via `Close`))

(event `self.ReceiveAnyDamage`
  (params (Damage :type "Float (single-precision)") (DamageType :type "DamageType Object Reference") (InstigatedBy :type "Controller Object Reference") (DamageCauser :type "Actor Object Reference"))
  (`/Game/CathodeArena/Core/Engine/BP_FunctionLibrary.LogErer` (`KismetStringLibrary.Conv_DoubleToString` Damage)))

(fn `UserConstructionScript`
  (`StaticMeshComponent.SetStaticMesh` (`self.BaseMesh`) (`self.Mesh`)))