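; Interactive TV projector, a child of a parent TV-style object, that mirrors its current channel onto a BP_Spot child actor.
; The construction script configures the inherited channel material settings and caches the spot reference.
; UpdateSpot copies the Texture and Time parameters from the channel material to the spot as channel and speed.
; It refreshes on construction, BeginPlay, punches and channel changes, after the parent logic runs.
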(event `self.ReceiveBeginPlay`
  (`parent.ReceiveBeginPlay`)
  (`self.UpdateSpot` :!label _label))

(event `/Game/CathodeArena/Core/PhysicActors/BP_InteractiveObject.Punched`
  (params (Direction :type "Vector Structure") (Impulse :type "Float (single-precision)"))
  (`parent.Punched` Direction Impulse)
  (goto _label))

(event `self.JustChangeChannel`
  (params (HandLeft :type Boolean))
  (`parent.JustChangeChannel` false)
  (goto _label))

(fn `UpdateSpot`
  (bind _m_channel (`self.M_Channel`))
  (bind _pspot (`self.pSpot`))
  (bind _returnvalue (`MaterialInstanceDynamic.K2_GetTextureParameterValue` _m_channel "Texture"))
  (`/Game/CathodeArena/Core/Environment/BP_Spot.SetSpotChannel` _pspot _returnvalue)
  (bind _returnvalue_2 (`MaterialInstanceDynamic.K2_GetScalarParameterValue` _m_channel "Time"))
  (`/Game/CathodeArena/Core/Environment/BP_Spot.SetSpotSpeed` _pspot _returnvalue_2))

(fn `UserConstructionScript`
  (set `self.MeshChannelMatID` 1)
  (set `self.Reverse` true)
  (`parent.UserConstructionScript`)
  ;[1 1 1] ref Spot
  (set `self.pSpot` (cast `/Game/CathodeArena/Core/Environment/BP_Spot` (`ChildActorComponent.ChildActor` (`self.BP_Spot`)) :!pure true))
  (`self.UpdateSpot`))