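; Interactive TV physics actor that shows animated GIF textures on its screen and switches channel when hit.
; Construction creates a dynamic screen material, optionally from a reversed instance, with an initial speed and either a random GIF or a hand-set texture, reapplied on BeginPlay.
; A punch picks a random GIF, while JustChangeChannel delegates to ChangeChannel with the material and hand.
; Both events then randomize playback speed through the material's Time parameter.
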(event `self.ReceiveBeginPlay`
  (`parent.ReceiveBeginPlay`)
  (`self.SetGifRandomOrNot`))

(event `self.Punched`
  (params (Direction :type "Vector Structure") (Impulse :type "Float (single-precision)"))
  (bind _allgifs (`/Game/CathodeArena/Core/Engine/BP_FunctionLibrary.GetAllGifs`))
  (`parent.Punched` Direction Impulse)
  (`MaterialInstanceDynamic.SetTextureParameterValue` (`self.DMI_Channel`) "Texture" (`|GetArrayItem` _allgifs (`KismetMathLibrary.RandomIntegerInRange` 0 (`KismetArrayLibrary.Array_LastIndex` _allgifs))))
  (`self.SetGifSpeed` (`KismetMathLibrary.RandomFloatInRange` 1.0 20.0) :!label _label))

(event `JustChangeChannel`
  (params (HandLeft :type Boolean))
  (`/Game/CathodeArena/Core/Engine/BP_FunctionLibrary.ChangeChannel` (`self.DMI_Channel`) HandLeft)
  (goto _label))

(fn `SetGifRandomOrNot`
  (bind _allgifs (`/Game/CathodeArena/Core/Engine/BP_FunctionLibrary.GetAllGifs`))
  (bind _t_channel (`self.T_Channel`))
  (if (`self.RandomGifAtStart`)
    ;[1 1 1] On overide la potentielle texture settée à la mano dans la scene
    (`MaterialInstanceDynamic.SetTextureParameterValue` (`self.DMI_Channel`) "Texture" (`|GetArrayItem` _allgifs (`KismetMathLibrary.RandomIntegerInRange` 0 (`KismetArrayLibrary.Array_LastIndex` _allgifs))))
    (else
      ;[1 1 1] Set texture si settée à la mano dans la scene
      (`/Engine/EditorBlueprintResources/StandardMacros.IsValid` _t_channel
        (:`Is Valid`
          (`MaterialInstanceDynamic.SetTextureParameterValue` (`self.DMI_Channel`) "Texture" _t_channel))))))

(fn `SetGifSpeed`
  (params (Value :type "Float (double-precision)"))
  (`MaterialInstanceDynamic.SetScalarParameterValue` (`self.DMI_Channel`) "Time" Value))

(fn `UserConstructionScript`
  (`parent.UserConstructionScript`)
  (bind _returnvalue (`PrimitiveComponent.CreateDynamicMaterialInstance` (`self.StaticMeshComponent`) (`self.MeshChannelMatID`) (select `bool` (`self.Reverse`) :`false` "/Game/CathodeArena/MaterialLibrary/Screens/M_Screen_Inst.M_Screen_Inst" :`true` "/Game/CathodeArena/MaterialLibrary/Screens/M_Screen_Inst_InstReverse.M_Screen_Inst_InstReverse" :!type "MaterialInterface Object Reference") "None"))
  (set `self.DMI_Channel` _returnvalue)
  (`self.SetGifSpeed` (`self.InitialGifSpeed`))
  (`self.SetGifRandomOrNot`))