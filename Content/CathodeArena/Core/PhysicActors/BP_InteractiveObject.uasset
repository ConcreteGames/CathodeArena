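; Physics prop that players can punch or throw, with mass adjusted and a random scale chance at spawn.
; Punches add to a stored impulse, launched immediately unless the prop is held, then reset by ThrowObject.
; Stored impulse drives a debug arrow and the play rate of a blink timeline meant to flash materials white.
; Punches and hits with enough upward velocity trigger sounds, the latter rate-limited.
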(event `self.ReceiveBeginPlay`
  ;[0 1 0.09869] BEGIN PLAY
  (cast `/Game/CathodeArena/Core/PhysicActors/BP_I_PinballBall` self
    (:`then`
      (`PrimitiveComponent.SetMassOverrideInKg` (`self.StaticMeshComponent`) "None" (/ (`PrimitiveComponent.GetMass` (`self.StaticMeshComponent`)) 2.0) true))
    (:`CastFailed`
      ;[1 1 1] Clamp Mass
      (`PrimitiveComponent.SetMassOverrideInKg` (`self.StaticMeshComponent`) "None" (`KismetMathLibrary.FClamp` (`PrimitiveComponent.GetMass` (`self.StaticMeshComponent`)) 0.0 1000.0) true)))
  ;[1 1 1] Add random scale probability
  (`/Game/CathodeArena/Core/Engine/BP_FunctionLibrary.AddRandomScaleProba` self (`self.RandomScaleDiffPercentage`))
  (`self.SaveMaterials`)
  (`self.InitBlink`))

(event `AddNextThrowForce`
  (params (ImpulseToAdd :type "Float (double-precision)"))
  (bind _throwimpulse (`/Game/CathodeArena/Core/Characters/BP_GravityCharacterBase.ThrowImpulse` (`/Game/CathodeArena/Core/Engine/BP_FunctionLibrary.GetChar`)))
  (set `self.NextThrowImpulse` (+ (`self.NextThrowImpulse`) ImpulseToAdd))
  (`TimelineComponent.SetPlayRate` (`self.T_Blink`) (`KismetMathLibrary.MapRangeClamped` (`self.NextThrowImpulse`) _throwimpulse (* _throwimpulse 100.0) 1.0 50.0))
  (`self.UpdateArrow`))

(event `Punched`
  (params (Direction :type "Vector Structure") (Impulse :type "Float (double-precision)"))
  (set `self.ThrowDirection` Direction)
  (`self.AddNextThrowForce` Impulse)
  (if (not (`self.IsPickedUp`))
    (`self.ThrowObject` false))
  ;[1 1 1] blink un coup
  (`TimelineComponent.PlayFromStart` (`self.T_Blink`))
  (`self.OnPunched`))

(event `ThrowObject`
  (params (OverideDirection :type Boolean) (NewDirection :type "Vector Structure"))
  (bind _staticmeshcomponent (`self.StaticMeshComponent`))
  (if OverideDirection
    (set `self.ThrowDirection` NewDirection))
  (`PrimitiveComponent.SetPhysicsLinearVelocity` _staticmeshcomponent (0.0 0.0 0.0) true "None")
  (`PrimitiveComponent.AddImpulse` _staticmeshcomponent (* (`self.ThrowDirection`) (`self.NextThrowImpulse`)) "None" false)
  ;[1 1 1] reset Impulse
  (set `self.NextThrowImpulse` 0.0)
  (`self.UpdateArrow`)
  (`PrimitiveComponent.SetCollisionResponseToChannel` _staticmeshcomponent "ECC_Pawn" "ECR_Block")
  (set `self.IsPickedUp` false))

(event `InitBlink`
  (bind _t_blink (`self.T_Blink`))
  (`TimelineComponent.SetTimelineLength` _t_blink 0.5)
  (`TimelineComponent.SetPlayRate` _t_blink 1.0))

(event `self.StaticMeshComponent.OnComponentHit`
  (params (HitComponent :type "PrimitiveComponent Object Reference") (OtherActor :type "Actor Object Reference") (OtherComp :type "PrimitiveComponent Object Reference") (NormalImpulse :type "Vector Structure") (Hit :type "HitResult Structure (by ref)"))
  ;[1 1 1] WIP
  (`self.Sound`))

(event `Sound`
  (bind (_returnvalue_x _returnvalue_y _returnvalue_z) (`KismetMathLibrary.BreakVector` (`self.GetVelocity`)))
  (if (>= _returnvalue_z 100.0)
    (`self.GateForSound` 0.2
      (:`Play`
        (`FMODBlueprintStatics.PlayEventAtLocation` "/Game/FMOD/Events/Envir/ENV_PropsHitGround.ENV_PropsHitGround" (`self.GetTransform`))))))

(event `OpenSoundGate`
  ;[1 1 1] Sound
  (`/Engine/EditorBlueprintResources/StandardMacros.Gate` false :!via `Open` :!label _label
    (:`Exit`
      (`FMODBlueprintStatics.PlayEvent2D` "/Game/FMOD/Events/Gameplay/ENV_Hit.ENV_Hit")
      (`self.CloseSoundGate`)
      (`KismetSystemLibrary.Delay` 0.2)
      (`self.OpenSoundGate`))))

(event `CloseSoundGate`
  ;[1 1 1] Sound
  (goto _label :!via `Close`))

(event `OnPunched`
  (`FMODBlueprintStatics.PlayEvent2D` "/Game/FMOD/Events/Gameplay/ENV_Hit.ENV_Hit"))

(fn `ResetMaterial`
  (params (ElementIndex :type Integer) (Material :type "MaterialInterface Object Reference"))
  (`PrimitiveComponent.SetMaterial` (`self.StaticMeshComponent`) ElementIndex Material))

(fn `SaveMaterials`
  (bind _staticmeshcomponent (`self.StaticMeshComponent`))
  (for _index (range (`PrimitiveComponent.GetNumMaterials` _staticmeshcomponent))
    (`KismetArrayLibrary.Array_Add` (`self.InitialMATs`) (`PrimitiveComponent.GetMaterial` _staticmeshcomponent _index))))

(fn `UpdateArrow`
  (bind _nextthrowimpulse (`self.NextThrowImpulse`))
  (bind _debug_newthrowvector (`self.DEBUG_NewThrowVector`))
  (`SceneComponent.SetWorldScale3D` _debug_newthrowvector (`KismetMathLibrary.MakeVector` _nextthrowimpulse _nextthrowimpulse _nextthrowimpulse))
  (`SceneComponent.K2_SetWorldRotation` _debug_newthrowvector (`KismetMathLibrary.FindLookAtRotation` (0.0 0.0 0.0) (`self.ThrowDirection`)) false false))

(fn `UserConstructionScript`)