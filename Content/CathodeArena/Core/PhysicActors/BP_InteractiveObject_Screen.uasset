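; Punchable screen prop that shows a random animated texture through a BP_LightingScreens child actor.
; The construction script picks a texture from AllGifs, passes it with light, timing, projection and scale settings to the child, then calls its Constructor to apply them.
; Each punch usually unhides the screen and switches to a random texture the same way, with a smaller chance of hiding it to simulate switching off.
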(event `self.Punched`
  (params (Direction :type "Vector Structure") (Impulse :type "Float (single-precision)"))
  (`parent.Punched` Direction Impulse)
  (if (`KismetMathLibrary.RandomBoolWithWeight` 0.75)
    (`self.SwitchToAnotherChannel`)
    (else
      (`self.SwitchOff`))))

(event `SwitchToAnotherChannel`
  (bind _allgifs (`self.AllGifs`))
  (bind _asbp_lighting_screens (cast `/Game/CathodeArena/Core/Environment/BP_LightingScreens` (`ChildActorComponent.ChildActor` (`self.BP_LightingScreens`)) :!pure true))
  (`SceneComponent.SetHiddenInGame` (`self.BP_LightingScreens`) false false)
  (set `self.CurrentGif` (`|GetArrayItem` _allgifs (`KismetMathLibrary.RandomIntegerInRange` 0 (`KismetArrayLibrary.Array_LastIndex` _allgifs))))
  (set `/Game/CathodeArena/Core/Environment/BP_LightingScreens.MidTexture` (`self.CurrentGif`) _asbp_lighting_screens)
  (`/Game/CathodeArena/Core/Environment/BP_LightingScreens.Constructor` _asbp_lighting_screens))

(event `SwitchOff`
  (`SceneComponent.SetHiddenInGame` (`self.BP_LightingScreens`) true false))

(fn `UserConstructionScript`
  (bind _allgifs (`self.AllGifs`))
  (`parent.UserConstructionScript`)
  (set `self.MidTexture` (`|GetArrayItem` _allgifs (`KismetMathLibrary.RandomIntegerInRange` 0 (`KismetArrayLibrary.Array_LastIndex` _allgifs))))
  (bind _asbp_lighting_screens (cast `/Game/CathodeArena/Core/Environment/BP_LightingScreens` (`ChildActorComponent.ChildActor` (`self.BP_LightingScreens`))))
  (set `/Game/CathodeArena/Core/Environment/BP_LightingScreens.AttenuationRadius` (`self.LightAttenuation`) _asbp_lighting_screens)
  (set `/Game/CathodeArena/Core/Environment/BP_LightingScreens.Intensity` (`self.Intensity`) _asbp_lighting_screens)
  (set `/Game/CathodeArena/Core/Environment/BP_LightingScreens.OuterConeAngle` (`self.OuterCone`) _asbp_lighting_screens)
  (set `/Game/CathodeArena/Core/Environment/BP_LightingScreens.MidTexture` (`self.MidTexture`) _asbp_lighting_screens)
  (set `/Game/CathodeArena/Core/Environment/BP_LightingScreens.Time` (`self.Time`) _asbp_lighting_screens)
  (set `/Game/CathodeArena/Core/Environment/BP_LightingScreens.ScreenScale` (* (`self.GetActorScale3D`) (`self.ScreenScale`)) _asbp_lighting_screens)
  (set `/Game/CathodeArena/Core/Environment/BP_LightingScreens.EmitProjection` (`self.EmitProjection`) _asbp_lighting_screens)
  (`/Game/CathodeArena/Core/Environment/BP_LightingScreens.Constructor` _asbp_lighting_screens))