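; BP_GameMode is a game mode Blueprint that keeps a running "Bordel" total and broadcasts it to actors in the level.
; On BeginPlay, RefActors caches every actor implementing the BPI_Game interface in BordelActors.
; IncrementBordel adds the incoming amount to BordelAmount, then sends the new total to each cached actor through BordelMessage.
; Actors spawned after BeginPlay are not added to the list.
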(event `self.ReceiveBeginPlay`
  (`self.RefActors`))

(event `/Game/CathodeArena/Core/Engine/BPI_Game.IncrementBordel`
  (params (AddBordel :type Integer))
  ;[1 1 1] Increment Bordel from BPI_Game Actors
  (set `self.BordelAmount` (+ AddBordel (`self.BordelAmount`)))
  (for _array_element (`self.BordelActors`)
    (message `/Game/CathodeArena/Core/Engine/BPI_Game.Bordel` _array_element (`self.BordelAmount`))))

(fn `RefActors`
  (bind _outactors (`GameplayStatics.GetAllActorsWithInterface` "/Game/CathodeArena/Core/Engine/BPI_Game.BPI_Game_C"))
  (for _array_element _outactors
    (`KismetArrayLibrary.Array_Add` (`self.BordelActors`) _array_element)))

(fn `UserConstructionScript`)