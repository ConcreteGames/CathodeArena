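; Destructible glass screen Blueprint that displays channel images on an emissive material, with a tutorial variant.
; The construction script creates a dynamic screen material on a slot chosen by the tutorial flag, then applies either a random GIF texture or a hand-set channel texture.
; In tutorial mode it also sets a transparent black material on the regular screen slot.
; Outside tutorial mode, the triggered action changes the channel, passing along which hand acted.
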(event `/Game/CathodeArena/Core/Engine/BPI_Actionable.ActionTriggered`
  (params (HandIsLeft :type Boolean))
  (`self.IfTuto`
    (:`False`
      (`/Game/CathodeArena/Core/Engine/BP_FunctionLibrary.ChangeChannel` (`self.DMI_Channel`) HandIsLeft))))

(event `self.ReceiveBeginPlay`
  (`parent.ReceiveBeginPlay`))

(fn `RandomGifOrNot`
  (bind _allgifs (`/Game/CathodeArena/Core/Engine/BP_FunctionLibrary.GetAllGifs`))
  (bind _t_channel (`self.T_Channel`))
  (if (`self.RandomGifAtStart`)
    ;[1 1 1] On overide la potentielle texture settée à la mano dans la scene
    (`MaterialInstanceDynamic.SetTextureParameterValue` (`self.DMI_Channel`) "Texture" (`|GetArrayItem` _allgifs (`KismetMathLibrary.RandomIntegerInRange` 0 (`KismetArrayLibrary.Array_LastIndex` _allgifs))))
    (else
      ;[1 1 1] Set texture si settée à la mano dans la scene
      (`/Engine/EditorBlueprintResources/StandardMacros.IsValid` _t_channel
        (:`Is Valid`
          (`MaterialInstanceDynamic.SetTextureParameterValue` (`self.DMI_Channel`) "Texture" _t_channel))))))

(fn `UserConstructionScript`
  (`parent.UserConstructionScript`)
  (bind _returnvalue (`PrimitiveComponent.CreateDynamicMaterialInstance` (`self.Destructible`) (select `bool` (`self.IsTuto`) :`false` 3 :`true` 2) "/Game/CathodeArena/MaterialLibrary/Screens/M_Screen_InstEmissive.M_Screen_InstEmissive" "None"))
  (set `self.DMI_Channel` _returnvalue)
  (`self.RandomGifOrNot`)
  (`self.IfTuto`
    (:`True`
      (`PrimitiveComponent.SetMaterial` (`self.Destructible`) 3 "/Game/CathodeArena/Core/Destructibles/GlassTuto/M_TransBlack_Inst.M_TransBlack_Inst"))))