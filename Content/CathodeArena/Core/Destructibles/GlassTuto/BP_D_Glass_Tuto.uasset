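; BP_D_Glass_Tuto is a destructible glass tutorial actor that shows one hand-gesture tutorial UI until the glass breaks.
; The construction script uses the HandsStyle enum to unhide the matching component: grab, punch, finger, photo, reset, or general for the empty style.
; BeginPlay gathers all six tutorial components into an array, which is destroyed component by component when the Destructible fractures.
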(event `self.ReceiveBeginPlay`
  (`parent.ReceiveBeginPlay`)
  (set `self.AllTutos` (`|MakeArray` (`self.UI_TutoPunch`) (`self.UI_TutoFinger`) (`self.UI_TutoReset`) (`self.UI_TutoPhoto`) (`self.UI_TutoGeneral`) (`self.UI_TutoGrab`))))

(event `self.Destructible.OnComponentFracture`
  (params (HitPoint :type "Vector Structure (by ref)") (HitDirection :type "Vector Structure (by ref)"))
  (for _array_element (`self.AllTutos`)
    (`/Engine/EditorBlueprintResources/StandardMacros.IsValid` _array_element
      (:`Is Valid`
        (`ActorComponent.K2_DestroyComponent` _array_element)))))

(fn `UserConstructionScript`
  (`parent.UserConstructionScript`)
  (`SceneComponent.SetHiddenInGame` (select `/Game/CathodeArena/Core/Characters/HandsStyle` (`self.HandsStyle`) :`NewEnumerator0` (`self.UI_TutoGrab`) :`NewEnumerator1` (`self.UI_TutoPunch`) :`NewEnumerator2` (`self.UI_TutoFinger`) :`NewEnumerator3` (`self.UI_TutoPhoto`) :`NewEnumerator5` (`self.UI_TutoReset`) :`NewEnumerator6` (`self.UI_TutoGeneral`) :!type "SceneComponent Object Reference") false false))