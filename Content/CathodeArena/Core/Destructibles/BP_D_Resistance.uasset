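; BP_D_Resistance is a destructible resistor prop for CathodeArena, with randomly colored bands.
; Its construction script runs the parent's, then calls AddRandomRot90degree on itself to vary orientation.
; It then creates dynamic instances of M_ResistanceBande on the Destructible component's band material slots, giving each a random RGB Color.
; The event graph holds only disabled placeholder events, so all variation comes from construction.
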(fn `UserConstructionScript`
  (`parent.UserConstructionScript`)
  (`/Game/CathodeArena/Core/Engine/BP_FunctionLibrary.AddRandomRot90degree` self)
  ;[1 1 1] Random bandes color
  (for _index (range 2 6)
    (bind _returnvalue (`PrimitiveComponent.CreateDynamicMaterialInstance` (`self.Destructible`) _index "/Game/CathodeArena/Art/Props/Resistance/M_ResistanceBande.M_ResistanceBande" "None"))
    (`MaterialInstanceDynamic.SetVectorParameterValue` _returnvalue "Color" (make `LinearColor` (`KismetMathLibrary.RandomFloatInRange` 0.0 1.0) (`KismetMathLibrary.RandomFloatInRange` 0.0 1.0) (`KismetMathLibrary.RandomFloatInRange` 0.0 1.0) 1.0))))