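; Parent Blueprint for breakable props that get a random scale, take point damage and add to the game mode's "Bordel" counter when fractured.
; Hits accumulate damage, feed the Destructible component and shake dynamic materials through timeline-sampled curves, with power scaled by damage.
; Fracture plays glass or generic break audio.
; A hop and player-homing Tick sit behind a start-closed DoOnce with no reset, so appear dormant.
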(event `self.ReceiveBeginPlay`
  (bind _asbp_gravity_character_base (cast `/Game/CathodeArena/Core/Characters/BP_GravityCharacterBase` (`GameplayStatics.GetPlayerPawn` 0)))
  (set `self.pChar` _asbp_gravity_character_base)
  (`/Game/CathodeArena/Core/Engine/BP_FunctionLibrary.AddRandomScaleProba` self (`self.RandomScalePercentage`)))

(event `self.ReceiveTick`
  (params (DeltaSeconds :type "Float (single-precision)"))
  (bind _returnvalue (`self.K2_GetActorLocation`))
  ;[1 1 1] à quoi ça sert ?
  (if (`self.IsAwake`)
    (`self.K2_SetActorLocation` (+ (* (* (`KismetMathLibrary.Normal` (- (`self.K2_GetActorLocation` (`self.pChar`)) _returnvalue)) (`GameplayStatics.GetWorldDeltaSeconds`)) 100.0) _returnvalue))))

(event `self.ReceivePointDamage`
  (params (Damage :type "Float (single-precision)") (DamageType :type "DamageType Object Reference") (HitLocation :type "Vector Structure") (HitNormal :type "Vector Structure") (HitComponent :type "PrimitiveComponent Object Reference") (BoneName :type Name) (ShotFromDirection :type "Vector Structure") (InstigatedBy :type "Controller Object Reference") (DamageCauser :type "Actor Object Reference") (HitInfo :type "HitResult Structure (by ref)"))
  (bind (_returnvalue_x _returnvalue_y _returnvalue_z) (`KismetMathLibrary.BreakVector` (`self.K2_GetActorLocation`)))
  ;[1 1 1] Event Point Damage
  (`self.AddDamage` Damage)
  (`FMODBlueprintStatics.PlayEvent2D` "/Game/FMOD/Events/Gameplay/ENV_Hit.ENV_Hit")
  (`DestructibleComponent.ApplyDamage` (`self.Destructible`) (`self.Damage`) HitLocation ShotFromDirection 0.0)
  (`self.ShakeDatMesh`)
  (`/Engine/EditorBlueprintResources/StandardMacros.DoOnce` true
    (:`Completed`
      (set `self.IsAwake` true)
      (bind (_direction _position) (`Timeline|Jumping` :!via `PlayFromStart`)
        (:`Update`
          (bind _returnvalue (* _position 5.0))
          (`self.K2_SetActorLocation` (`KismetMathLibrary.MakeVector` _returnvalue_x (select `bool` (`KismetMathLibrary.RandomBoolWithWeight` 0.5) :`false` (+ _returnvalue_y _returnvalue) :`true` (- _returnvalue_y _returnvalue)) (+ _returnvalue_z (* _position 20.0)))))))))

(event `self.Destructible.OnComponentHit`
  (params (HitComponent :type "PrimitiveComponent Object Reference") (OtherActor :type "Actor Object Reference") (OtherComp :type "PrimitiveComponent Object Reference") (NormalImpulse :type "Vector Structure") (Hit :type "HitResult Structure (by ref)")))

(event `ShakeDatMesh`
  ;[1 1 1] Shake The Mesh When Hit
  (`TimelineComponent.SetTimelineLength` (`self.ShakeDatMeshAndMaterial`) (`self.ShakeTimelineLength`))
  (`Timeline|ShakeDatMeshAndMaterial` :!via `PlayFromStart`
    (:`Update`
      (`self.ShakeDatMaterial` (`CurveFloat.GetFloatValue` (`self.CurveShake`) (`/Game/CathodeArena/Core/Engine/BP_FunctionLibrary.GetTimelinePercentage` (`self.ShakeDatMeshAndMaterial`))) (* (`CurveFloat.GetFloatValue` (`self.CurveShakeTime`) (`/Game/CathodeArena/Core/Engine/BP_FunctionLibrary.GetTimelinePercentage` (`self.ShakeDatMeshAndMaterial`))) 2.0) (* (`CurveFloat.GetFloatValue` (`self.CurveShakePower`) (`/Game/CathodeArena/Core/Engine/BP_FunctionLibrary.GetTimelinePercentage` (`self.ShakeDatMeshAndMaterial`))) (`KismetMathLibrary.MapRangeClamped` (`self.Damage`) 0.0 10000.0 5.0 20.0))))))

(event `self.Destructible.OnComponentFracture`
  (params (HitPoint :type "Vector Structure (by ref)") (HitDirection :type "Vector Structure (by ref)"))
  (bind _returnvalue (`self.GetTransform`))
  (cast `/Game/CathodeArena/Core/Destructibles/BP_D_Glass` self
    (:`then`
      (`FMODBlueprintStatics.PlayEventAtLocation` "/Game/FMOD/Events/Envir/ENV_PropsGlassBreak.ENV_PropsGlassBreak" _returnvalue))
    (:`CastFailed`
      (`FMODBlueprintStatics.PlayEventAtLocation` "/Game/FMOD/Events/Envir/ENV_PropsBreak.ENV_PropsBreak" _returnvalue)))
  (`/Game/CathodeArena/Core/GameModes/BP_GameMode.IncrementBordel` (`/Game/CathodeArena/Core/Engine/BP_FunctionLibrary.GetGM`) (`self.BordelToAdd`)))

(fn `AddDamage`
  (params (DamagePoints :type "Float (double-precision)"))
  (set `self.Damage` (+ DamagePoints (`self.Damage`))))

(fn `ShakeDatMaterial`
  (params (Shake :type "Float (double-precision)") (TimeMultiple :type "Float (double-precision)") (Power :type "Float (double-precision)"))
  (for _array_element (`self.MID`)
    (`MaterialInstanceDynamic.SetScalarParameterValue` _array_element "Shake" Shake)
    (`MaterialInstanceDynamic.SetScalarParameterValue` _array_element "TimeMultiple" (`local.TimeMultiple`))
    (`MaterialInstanceDynamic.SetScalarParameterValue` _array_element "Power" (`local.Power`))))

(fn `UserConstructionScript`
  (bind _destructible (`self.Destructible`))
  (`PrimitiveComponent.SetEnableGravity` (`self.Destructible`) (`self.EnableGravity`))
  (`DestructibleComponent.SetDestructibleMesh` _destructible (`self.DMToSet`))
  (for (_array_element _array_index) (`MeshComponent.GetMaterials` _destructible)
    (bind _returnvalue (`PrimitiveComponent.CreateDynamicMaterialInstance` (`self.Destructible`) _array_index _array_element "None"))
    (`KismetArrayLibrary.Array_AddUnique` (`self.MID`) _returnvalue)))