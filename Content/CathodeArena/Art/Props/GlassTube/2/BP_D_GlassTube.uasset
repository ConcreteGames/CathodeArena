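; Destructible glass tube prop for the Cathode Arena that switches off a gravity volume when it breaks.
; When its Destructible component fractures, it finds all BP_GravityVolumeBox actors in the level and destroys the first one returned.
; The link is a global class lookup rather than a direct reference, and the construction script adds nothing beyond the parent's.
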(event `self.Destructible.OnComponentFracture`
  (params (HitPoint :type "Vector Structure (by ref)") (HitDirection :type "Vector Structure (by ref)"))
  (bind _outactors (`GameplayStatics.GetAllActorsOfClass` "/Game/DirectionalGravity/Blueprints/SceneObjects/BP_GravityVolumeBox.BP_GravityVolumeBox_C"))
  (`self.K2_DestroyActor` (`|GetArrayItem` _outactors)))

(fn `UserConstructionScript`
  (`parent.UserConstructionScript`))