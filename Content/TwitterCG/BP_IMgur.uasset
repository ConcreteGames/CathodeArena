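; Screenshot-to-tweet actor for Stunfest 2019, with extra ConcreteMode-gated hotkeys for BugScreenShot and HighResShot captures.
; T pauses the game and opens WBP_Twitter.
; CommitText replaces the last BugIt screenshot, unpauses and POSTs the PNG to a hardcoded server behind a loading widget.
; Success opens a Twitter URL with a random catchphrase, hashtags and Imgur link parsed from the response, while failure briefly shows a connection error.
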(event `self.ReceiveBeginPlay`
  (`self.EnableInput` (`GameplayStatics.GetPlayerController` 0)))

(event `Key|B`
  (params (Key :type "Key Structure"))
  (:`Pressed`
    (`/Game/CathodeArena/Core/BP_MacroLibrary.ConcreteMode` :!label _label
      (:`TRUE`
        (`KismetSystemLibrary.ExecuteConsoleCommand` (`KismetStringLibrary.Concat_StrStr` "BugScreenShot") null)))))

(event `Key|M`
  (params (Key :type "Key Structure"))
  (:`Pressed`
    (goto _label)))

(event `Key|NumPadOne`
  (params (Key :type "Key Structure"))
  (:`Pressed`
    (`/Game/CathodeArena/Core/BP_MacroLibrary.ConcreteMode`
      (:`TRUE`
        (`KismetSystemLibrary.ExecuteConsoleCommand` (`KismetStringLibrary.Concat_StrStr` "HighResShot " "1") null)))))

(event `Key|H`
  (params (Key :type "Key Structure"))
  (:`Pressed`
    (`/Game/CathodeArena/Core/BP_MacroLibrary.ConcreteMode`
      (:`TRUE`
        (`KismetSystemLibrary.ExecuteConsoleCommand` (`KismetStringLibrary.Concat_StrStr` "HighResShot " "1920x1080") null)))))

(event `Key|NumPadTwo`
  (params (Key :type "Key Structure"))
  (:`Pressed`
    (`/Game/CathodeArena/Core/BP_MacroLibrary.ConcreteMode`
      (:`TRUE`
        (`KismetSystemLibrary.ExecuteConsoleCommand` (`KismetStringLibrary.Concat_StrStr` "HighResShot " "2") null)))))

(event `Key|J`
  (params (Key :type "Key Structure"))
  (:`Pressed`
    (`/Game/CathodeArena/Core/BP_MacroLibrary.ConcreteMode`
      (:`TRUE`
        (`KismetSystemLibrary.ExecuteConsoleCommand` (`KismetStringLibrary.Concat_StrStr` "HighResShot " "1080x1920") null)))))

(event `Key|NumPadThree`
  (params (Key :type "Key Structure"))
  (:`Pressed`
    (`/Game/CathodeArena/Core/BP_MacroLibrary.ConcreteMode`
      (:`TRUE`
        (`KismetSystemLibrary.ExecuteConsoleCommand` (`KismetStringLibrary.Concat_StrStr` "HighResShot " "3") null)))))

(event `Key|K`
  (params (Key :type "Key Structure"))
  (:`Pressed`
    (`/Game/CathodeArena/Core/BP_MacroLibrary.ConcreteMode`
      (:`TRUE`
        (`KismetSystemLibrary.ExecuteConsoleCommand` (`KismetStringLibrary.Concat_StrStr` "HighResShot " "9324x5265") null)))))

(event `Key|NumPadFour`
  (params (Key :type "Key Structure"))
  (:`Pressed`
    (`/Game/CathodeArena/Core/BP_MacroLibrary.ConcreteMode`
      (:`TRUE`
        (`KismetSystemLibrary.ExecuteConsoleCommand` (`KismetStringLibrary.Concat_StrStr` "HighResShot " "4") null)))))

(event `Key|NumPadFive`
  (params (Key :type "Key Structure"))
  (:`Pressed`
    (`/Game/CathodeArena/Core/BP_MacroLibrary.ConcreteMode`
      (:`TRUE`
        (`KismetSystemLibrary.ExecuteConsoleCommand` (`KismetStringLibrary.Concat_StrStr` "HighResShot " "5") null)))))

(event `Key|L`
  (params (Key :type "Key Structure"))
  (:`Pressed`
    (`/Game/CathodeArena/Core/BP_MacroLibrary.ConcreteMode`
      (:`TRUE`
        (`KismetSystemLibrary.ExecuteConsoleCommand` (`KismetStringLibrary.Concat_StrStr` "HighResShot " "5265x9324") null)))))

(event `Key|NumPadSix`
  (params (Key :type "Key Structure"))
  (:`Pressed`
    (`/Game/CathodeArena/Core/BP_MacroLibrary.ConcreteMode`
      (:`TRUE`
        (`KismetSystemLibrary.ExecuteConsoleCommand` (`KismetStringLibrary.Concat_StrStr` "HighResShot " "6") null)))))

(event `Key|NumPadSeven`
  (params (Key :type "Key Structure"))
  (:`Pressed`
    (`/Game/CathodeArena/Core/BP_MacroLibrary.ConcreteMode`
      (:`TRUE`
        (`KismetSystemLibrary.ExecuteConsoleCommand` (`KismetStringLibrary.Concat_StrStr` "HighResShot " "7") null)))))

(event `Key|NumPadEight`
  (params (Key :type "Key Structure"))
  (:`Pressed`
    (`/Game/CathodeArena/Core/BP_MacroLibrary.ConcreteMode`
      (:`TRUE`
        (`KismetSystemLibrary.ExecuteConsoleCommand` (`KismetStringLibrary.Concat_StrStr` "HighResShot " "8") null)))))

(event `Key|NumPadNine`
  (params (Key :type "Key Structure"))
  (:`Pressed`
    (`/Game/CathodeArena/Core/BP_MacroLibrary.ConcreteMode`
      (:`TRUE`
        (`KismetSystemLibrary.ExecuteConsoleCommand` (`KismetStringLibrary.Concat_StrStr` "HighResShot " "9") null)))))

(event `Key|NumPadZero`
  (params (Key :type "Key Structure"))
  (:`Pressed`
    (`/Game/CathodeArena/Core/BP_MacroLibrary.ConcreteMode`
      (:`TRUE`
        (`KismetSystemLibrary.ExecuteConsoleCommand` (`KismetStringLibrary.Concat_StrStr` "HighResShot " "10") null)))))

(event `Key|T`
  (params (Key :type "Key Structure"))
  (:`Pressed`
    (if (not (`self.WanaTweet`))
      (set `self.WanaTweet` true)
      (`self.CaptureAndShare`))))

(event `CaptureAndShare`
  (`self.Make Widget`))

(event `CommitText`
  (bind _returnvalue (`GameplayStatics.GetPlayerController` 0))
  (`self.DeleteLastScreenshot`)
  (`self.CaptureImage` "0.5")
  (`GameplayStatics.SetGamePaused` false)
  (`LowEntryExtendedStandardLibrary.DelayFrames` 5)
  (`self.UploadToServer`)
  (`Widget.RemoveFromParent` (`self.Widget`))
  (`WidgetBlueprintLibrary.SetInputMode_GameOnly` _returnvalue)
  (set `PlayerController.bShowMouseCursor` false _returnvalue))

(event `DeleteLastScreenshot`
  (`LowEntryFileManagerFile.Delete` (`LowEntryFileManagerDirectory.GetFile` (`LowEntryFileManagerLibrary.GetDirectory` (select `bool` (`self.Mac`) :`false` "../../Saved/BugIt/WindowsNoEditor/" :`true` "../../Saved/BugIt/Mac/")) "BugScreenShot_00000.png")))

(event `CaptureImage`
  (params (Scale :type String :default "0.5"))
  ;[1 1 1] Scale 1 for player screen size, 0.5 for half, 2 for double
  (`KismetSystemLibrary.ExecuteConsoleCommand` "BugScreenShot" null))

(event `NoInternetCo`
  (params (Request :type "VaRestRequestJSON Object Reference"))
  (`self.ShowErrorCo`)
  (`KismetSystemLibrary.Delay` 3.0)
  (`self.HideErrorCo`)
  (set `self.WanaTweet` false))

(event `UploadToServer`
  (`self.ShowLoading`)
  (bind _output_get (set `self.Request` (`VaRestRequestJSON.ConstructRequestExt` "POST" "binary")))
  (`VaRestRequestJSON.SetBinaryRequestContent` _output_get (`LowEntryFileManagerFile.GetData` (select `bool` (`LowEntryExtendedStandardLibrary.WithEditor`) :`false` (`LowEntryFileManagerDirectory.GetFile` (`LowEntryFileManagerLibrary.GetDirectory` (select `bool` (`self.Mac`) :`false` "../../Saved/BugIt/WindowsNoEditor/" :`true` "../../Saved/BugIt/Mac/")) "BugScreenShot_00000.png") :`true` (`LowEntryFileManagerDirectory.GetFile` (`LowEntryFileManagerLibrary.GetDirectory` "C:\\UnrealProjects\\CathodeArena\\Saved\\BugIt\\Windows\\") "BugScreenShot_00000.png"))))
  (add `VaRestRequestJSON.OnRequestComplete` _output_get (delegate `Success`))
  (add `VaRestRequestJSON.OnRequestFail` _output_get (delegate `NoInternetCo`))
  ;[1 0 0.1534] server URL
  (`VaRestRequestJSON.ProcessURL` _output_get "http://51.15.205.111:6699/image/"))

(event `Success`
  (params (Request :type "VaRestRequestJSON Object Reference"))
  (`self.HideLoading`)
  (bind _returnvalue (`VaRestRequestJSON.GetResponseContentAsString` Request true))
  (`KismetSystemLibrary.LaunchURL` (`KismetStringLibrary.Concat_StrStr` (`self.StaticTwitterURL`) (select `int` (`KismetMathLibrary.RandomIntegerInRange` 0 20) :`0` "I'm ready for it!" :`1` "Come get some! " :`2` "The cake is a lie..." :`3` "Objection!" :`4` "Game is never over!" :`5` "Tu veux qu'on se tire l'oreille ?" :`6` "All your base are belong to us!" :`7` "FATALITY!" :`8` "Co-Co-Co-Combo Breaker!" :`9` "Fest is coming..." :`10` "Habile Bill !" :`11` "En ville, la loi, c'est toi. Ici c'est moi!" :`12` "I'll be back!" :`13` "C’est ça, la puissance intellectuelle. Bac + 2, les enfants!" :`14` "C'est pas banal..." :`15` "Où ça nous mène, la folie des hommes. On court tout droit à notre perte!" :`16` "Voilà, cadeau... de Noël !" :`17` "It's alive! It's alive!" :`18` "Nom de Zeus !" :`19` "Question de protocole..." :`20` "Houston on a un problème!") ";hashtags=Stunfest2019,StunfestMegaGlitch,rennes" " " (`KismetStringLibrary.Concat_StrStr` "https://imgur.com/" (`KismetStringLibrary.Split` (`KismetStringLibrary.Split` (`.RightS` (`KismetStringLibrary.Split` _returnvalue "/" "IgnoreCase" "FromEnd")) "\"") "."))))
  (`KismetSystemLibrary.Delay` 2.0)
  (set `self.WanaTweet` false))

(fn `HideErrorCo`
  (bind _ui_errorconnection (`self.UI_ErrorConnection`))
  (if (`Widget.IsInViewport` _ui_errorconnection)
    (`Widget.RemoveFromParent` _ui_errorconnection)))

(fn `HideLoading`
  (bind _ui_loading (`self.UI_Loading`))
  (if (`Widget.IsInViewport` _ui_loading)
    (`Widget.RemoveFromParent` _ui_loading)))

(fn `Make Widget`
  (bind _returnvalue (`GameplayStatics.GetPlayerController` 0))
  (`GameplayStatics.SetGamePaused` true)
  (bind _returnvalue_2 (`|CreateWidget` "/Game/TwitterCG/WBP_Twitter.WBP_Twitter_C"))
  (set `self.Widget` _returnvalue_2)
  (`UserWidget.AddToViewport` _returnvalue_2 0)
  (`WidgetBlueprintLibrary.SetInputMode_GameAndUIEx` _returnvalue _returnvalue_2)
  (set `PlayerController.bShowMouseCursor` true _returnvalue))

(fn `ShowErrorCo`
  (bind _ui_errorconnection (`self.UI_ErrorConnection`))
  (`self.HideLoading`)
  (`/Engine/EditorBlueprintResources/StandardMacros.IsValid` (`self.UI_ErrorConnection`)
    (:`Is Valid`
      _)
    (:`Is Not Valid`
      (bind _returnvalue (`|CreateWidget` "/Game/TwitterCG/UI_ErrorConnection.UI_ErrorConnection_C"))
      (set `self.UI_ErrorConnection` _returnvalue)))
  (if (not (`Widget.IsInViewport` _ui_errorconnection))
    (`UserWidget.AddToViewport` _ui_errorconnection 0)))

(fn `ShowLoading`
  (bind _ui_loading (`self.UI_Loading`))
  (`/Engine/EditorBlueprintResources/StandardMacros.IsValid` (`self.UI_Loading`)
    (:`Is Valid`
      _)
    (:`Is Not Valid`
      (bind _returnvalue (`|CreateWidget` "/Game/TwitterCG/UI_LoadingGif.UI_LoadingGif_C"))
      (set `self.UI_Loading` _returnvalue)))
  (if (not (`Widget.IsInViewport` _ui_loading))
    (`UserWidget.AddToViewport` _ui_loading 0)))

(fn `UserConstructionScript`)